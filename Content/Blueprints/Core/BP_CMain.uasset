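; Player controller that handles mouse input on the tile map, showing the cursor and caching the BP_TileMap actor at start.
; Left click queries the tile under the cursor without using the result.
; Right click asks the tile map for a path from CurrentTile to the tile under the cursor and only logs each step.
; CurrentTile is read but never set in this graph.
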(event `self.ReceiveBeginPlay`
  (set `self.bShowMouseCursor` true)
  (bind _returnvalue (`GameplayStatics.GetActorOfClass` "/Game/Blueprints/MainMode/BP_TileMap.BP_TileMap_C"))
  (set `self.TileMap` _returnvalue)
  (`self.EnableInput` self))

(event `self.ReceiveTick`
  (params (DeltaSeconds :type "Float (single-precision)")))

(event `Key|LeftMouseButton`
  (params (Key :type "Key Structure"))
  (:`Pressed`
    (`KismetSystemLibrary.PrintString` "Left" false)
    (`/Game/Blueprints/MainMode/BP_TileMap.GetTileUnderCursor` (`self.TileMap`))))

(event `Key|RightMouseButton`
  (params (Key :type "Key Structure"))
  (bind _currenttile_pos2d (break `TileInfo` (`self.CurrentTile`)))
  (bind _tilemap (`self.TileMap`))
  (bind _currenttile_pos2d_2 (break `TileInfo` (`self.CurrentTile`)))
  (:`Pressed`
    (`KismetSystemLibrary.PrintString` (`KismetStringLibrary.Concat_StrStr` "Right - " (`KismetStringLibrary.Conv_IntPointToString` _currenttile_pos2d)) false)
    (bind _tile (`/Game/Blueprints/MainMode/BP_TileMap.GetTileUnderCursor` _tilemap))
    (bind _returnvalue (`ActorTileMap.FindPath` _tilemap _currenttile_pos2d_2 (break `TileInfo` _tile)))
    (for _array_element _returnvalue
      (`KismetSystemLibrary.PrintString` (`KismetStringLibrary.Conv_IntPointToString` _array_element) false))))

(fn `UserConstructionScript`)