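; BP_PMain is a camera pawn with a spring arm for panning, rotating and zooming over a grid.
; Input sets target arm length, location and 45-degree rotation steps, which Tick eases toward with interpolation.
; Zoom is clamped to a fixed range, while forward and right movement clamp world Y and X using grid and viewport sizes.
; A cursor-trace debug print is left unconnected.
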(event `self.ReceiveBeginPlay`
  ;[1 1 1] BeginPlay
  (set `self.ZoomIterpolation` (`SpringArmComponent.TargetArmLength` (`self.SpringArm`)))
  (set `self.LocationInterpolation` (`self.K2_GetActorLocation`))
  (set `self.RotationInterpolation` (`self.K2_GetActorRotation`)))

(event `self.ReceiveTick`
  (params (DeltaSeconds :type "Float (single-precision)"))
  (bind _springarm (`self.SpringArm`))
  ;[1 1 1] TickUpdate
  (set `SpringArmComponent.TargetArmLength` (`KismetMathLibrary.FInterpTo` (`SpringArmComponent.TargetArmLength` _springarm) (`self.ZoomIterpolation`) DeltaSeconds 2.0) _springarm)
  (`self.K2_SetActorLocationAndRotation` (`KismetMathLibrary.VInterpTo` (`self.K2_GetActorLocation`) (`self.LocationInterpolation`) DeltaSeconds 5.0) (`KismetMathLibrary.RInterpTo` (`self.K2_GetActorRotation`) (`self.RotationInterpolation`) DeltaSeconds 5.0)))

(event `InputAxis|InputAxis_Zoom`
  (params (AxisValue :type "Float (single-precision)"))
  ;[1 1 1] Zoom
  (set `self.ZoomIterpolation` (`KismetMathLibrary.FClamp` (+ (* AxisValue 80.0) (`self.ZoomIterpolation`)) 80.0 2000.0)))

(event `InputAxis|InputAxis_Forward`
  (params (AxisValue :type "Float (single-precision)"))
  (bind (_grid_size_x _grid_size_y) (`KismetMathLibrary.BreakVector2D` (`/Game/Blueprints/Utilities/BPL_Utilities.GetGridSize`)))
  (bind (_returnvalue_x _returnvalue_y) (`KismetMathLibrary.BreakVector2D` (`WidgetLayoutLibrary.GetViewportSize`)))
  (bind (_returnvalue_x_2 _returnvalue_y_2 _returnvalue_z) (`KismetMathLibrary.BreakVector` (+ (`self.LocationInterpolation`) (* (`self.GetActorForwardVector`) (* AxisValue 30.0)))))
  ;[1 1 1] VerticalDisplacement
  (set `self.LocationInterpolation` (`KismetMathLibrary.MakeVector` _returnvalue_x_2 (`KismetMathLibrary.FClamp` _returnvalue_y_2 (* _returnvalue_y 1.5) _grid_size_y) _returnvalue_z)))

(event `InputAxis|InputAxis_Right`
  (params (AxisValue :type "Float (single-precision)"))
  (bind _grid_size_x (`KismetMathLibrary.BreakVector2D` (`/Game/Blueprints/Utilities/BPL_Utilities.GetGridSize`)))
  (bind _returnvalue_x (`KismetMathLibrary.BreakVector2D` (`WidgetLayoutLibrary.GetViewportSize`)))
  (bind _returnvalue (/ _returnvalue_x 3.0))
  (bind (_returnvalue_x_2 _returnvalue_y _returnvalue_z) (`KismetMathLibrary.BreakVector` (+ (`self.LocationInterpolation`) (* (`self.GetActorRightVector`) (* AxisValue 30.0)))))
  ;[1 1 1] LateralDisplacement
  (set `self.LocationInterpolation` (`KismetMathLibrary.MakeVector` (`KismetMathLibrary.FClamp` _returnvalue_x_2 _returnvalue (- _grid_size_x _returnvalue)) _returnvalue_y _returnvalue_z)))

(event `InputAction|InputAction_RotateRight`
  (params (Key :type "Key Structure"))
  ;[1 1 1] RightRotation
  (:`Pressed`
    (set `self.RotationInterpolation` (`KismetMathLibrary.ComposeRotators` (`self.RotationInterpolation`) (struct :`Yaw` -45.0)))))

(event `InputAction|InputAction_RotateLeft`
  (params (Key :type "Key Structure"))
  ;[1 1 1] LeftRotation
  (:`Pressed`
    (set `self.RotationInterpolation` (`KismetMathLibrary.ComposeRotators` (`self.RotationInterpolation`) (struct :`Yaw` 45.0)))))

(event `Key|LeftMouseButton`
  (params (Key :type "Key Structure")))

(fn `UserConstructionScript`)