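; Hex tile map actor that generates the world from game instance settings, spawns typed tile actors and syncs a child visual actor.
; It tracks which tiles carry each state and refreshes visuals on change, with cursor tracing and editor tile retyping.
; It also spawns units and settlements on tiles, binding their events back to itself to handle production, founding, resource gathering and unit destruction for the current faction.
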(event `self.ReceiveBeginPlay`
  (`self.SetActorTickEnabled` false)
  (`self.CalculateTileSize` "/Game/Assets/Models/HexTile.HexTile")
  (bind _asbp_ginstance (cast `/Game/Blueprints/Core/BP_GInstance` (`GameplayStatics.GetGameInstance`)))
  (`self.GenerateMap` (`GInstance.Size2D` _asbp_ginstance) (`GInstance.MapTemperature` _asbp_ginstance) (`GInstance.MapSeaLevel` _asbp_ginstance) (`GInstance.WaterTileChance` _asbp_ginstance))
  (`/Game/Blueprints/Core/GameElements/TileMap/BP_TileMapVisual.InitVisual` (`self.Visual`) self)
  (`self.DisplayMap`))

(event `self.ReceiveDestroyed`
  (for _array_element (`self.Tiles`)
    (`self.RemoveResourceFromTile` (`ActorTile.GetPos` _array_element))
    (`self.K2_DestroyActor` _array_element)))

(fn `AddStateToTile`
  (params (CurrTile :type "ActorTile Object Reference (by ref)") (TileStates :type "Array of ETileState Enum"))
  (for _array_element TileStates
    ;[0 0 0] Se obtienen las casillas con el estado dado y se anade la actual a la lista
    (bind _returnvalue (`self.GetTilesWithState` _array_element))
    (`KismetArrayLibrary.Array_Add` _returnvalue (`ActorTile.GetPos` (`local.CurrTile`)))
    (`BlueprintMapLibrary.Map_Add` (`self.TilesWithState`) _array_element (make `TilesArray` _returnvalue)))
  (`ActorTile.AddState` (`local.CurrTile`) (`local.TileStates`))
  (`self.UpdateTileVisual` (`local.CurrTile`)))

(fn `CalculateTileSize`
  (params (DefaultMesh :type "StaticMesh Object Reference"))
  (bind _returnvalue (`StaticMesh.GetBoundingBox` DefaultMesh))
  (bind _returnvalue_2 (* (.x (`.Max` (break `Box` _returnvalue))) (`KismetMathLibrary.Sqrt` 3.0)))
  (set `self.TileSize` (`KismetMathLibrary.MakeVector2D` (.x (`.Max` (break `Box` _returnvalue))) (.y (`.Max` (break `Box` _returnvalue)))))
  (set `self.HorizontalOffset` (+ (.x (`.Max` (break `Box` _returnvalue))) (/ (.x (`.Max` (break `Box` _returnvalue))) 2.0)))
  (set `self.VerticalOffset` _returnvalue_2)
  (set `self.RowOffset` (/ _returnvalue_2 2.0)))

(fn `ClearStateFromTiles`
  (params (State :type "ETileState Enum" :default "None"))
  (bind _returnvalue (`self.GetTilesWithState` State))
  (`BlueprintMapLibrary.Map_Remove` (`self.TilesWithState`) (`local.State`))
  (for _array_element _returnvalue
    (bind _returnvalue_2 (`self.GetTileAtPos` _array_element))
    (`/Engine/EditorBlueprintResources/StandardMacros.IsValid` _returnvalue_2
      (:`Is Valid`
        (`self.RemoveStateFromTile` _returnvalue_2 (`|MakeArray` (`local.State`)))))))

(fn `DisplayMap`
  (bind _values (`BlueprintMapLibrary.Map_Values` (`self.TilesInfo`)))
  (for _array_element _values
    (`self.DisplayTile` _array_element)))

(fn `DisplayTile`
  (params (Info :type "TileInfo Structure"))
  (bind (_pos2d _mappos2d _owner _type) (break `TileInfo` Info))
  (bind (_info_pos2d _info_mappos2d _info_owner _info_type _info_elements) (break `TileInfo` (`local.Info`)))
  (if (`|EnumInequality` _type)
    (`self.DisplayTileAtPos` (select `ETileType` _type :`Plains` "/Game/Blueprints/Core/GameElements/Tiles/BP_Tile_Plains.BP_Tile_Plains_C" :`Hills` "/Game/Blueprints/Core/GameElements/Tiles/BP_Tile_Hills.BP_Tile_Hills_C" :`Forest` "/Game/Blueprints/Core/GameElements/Tiles/BP_Tile_Forest.BP_Tile_Forest_C" :`SnowPlains` "/Game/Blueprints/Core/GameElements/Tiles/BP_Tile_Snow.BP_Tile_Snow_C" :`SnowHills` "/Game/Blueprints/Core/GameElements/Tiles/BP_Tile_Snow.BP_Tile_Snow_C" :`Ice` "/Game/Blueprints/Core/GameElements/Tiles/BP_Tile_Ice.BP_Tile_Ice_C" :`Mountains` "/Game/Blueprints/Core/GameElements/Tiles/BP_Tile_Mountains.BP_Tile_Mountains_C" :`Water` "/Game/Blueprints/Core/GameElements/Tiles/BP_Tile_Water.BP_Tile_Water_C" :!type "ActorTile Class Reference") (`local.Info`))
    (`/Game/Blueprints/Core/GameElements/TileMap/BP_TileMapVisual.UpdateVisual` (`self.Visual`) (make `TileInfo` _info_pos2d _info_mappos2d -1 _info_type _info_elements (`|MakeArray` "None" :!type "ETileState Enum")))))

(fn `GatherResource`
  (params (Pos2D :type "IntPoint Structure (by ref)"))
  (locals (Faction :type "/Game/Blueprints/MainMode/Core/BP_PFaction Object Reference") (TileInfo :type "TileInfo Structure"))
  (bind (_value _returnvalue) (`BlueprintMapLibrary.Map_Find` (`self.TilesInfo`) Pos2D))
  (if _returnvalue
    (bind _output_get (set `local.TileInfo` _value))
    (bind _asbp_smain (cast `/Game/Blueprints/MainMode/Core/BP_SMain` (`GameplayStatics.GetGameState`)))
    (bind _currentfaction (`SMain.CurrentFaction` _asbp_smain))
    (`/Engine/EditorBlueprintResources/StandardMacros.IsValid` _currentfaction
      (:`Is Valid`
        (bind _asbp_pfaction (cast `/Game/Blueprints/MainMode/Core/BP_PFaction` _currentfaction))
        (set `local.Faction` _asbp_pfaction)
        (bind ((`Resource` _resource)) (break `TileElements` (`.Elements` (break `TileInfo` _output_get))))
        (`/Engine/EditorBlueprintResources/StandardMacros.IsValid` _resource
          (:`Is Valid`
            (bind (_info_pos2d _info_owner _info_resource) (break `ResourceInfo` (`ActorResource.Info` _resource)))
            (`PawnFaction.AddResource` (`local.Faction`) _info_resource)
            (`ActorResource.SetFactionOwner` _resource (`PawnFaction.Index` (`local.Faction`)))))))))

(fn `GetTileUnderCursor`
  (returns (Tile :type "/Game/Blueprints/Core/GameElements/Tiles/BP_Tile Object Reference"))
  (bind _ascbase (cast `CBase` (`GameplayStatics.GetPlayerController` 0)))
  (bind (_hitresult _returnvalue) (`PlayerController.GetHitResultUnderCursorByChannel` _ascbase "TraceTypeQuery3" true))
  (if _returnvalue
    (bind _asbp_tile (cast `/Game/Blueprints/Core/GameElements/Tiles/BP_Tile` (`.HitActor` (`GameplayStatics.BreakHitResult` _hitresult))))
    (return _asbp_tile)
    (else
      (return null))))

(fn `InitUnit`
  (params (Faction :type "PawnFaction Object Reference") (Pos2D :type "IntPoint Structure (by ref)") (Unit :type "ProductionElement Structure (by ref)"))
  (locals (ActorUnit :type "ActorUnit Object Reference") (UnitInfo :type "UnitData Structure"))
  (bind (_unit_unit _unit_unittype) (break `ProductionElement` (`local.Unit`)))
  (bind (_value _returnvalue) (`BlueprintMapLibrary.Map_Find` (`self.TilesInfo`) (`local.Pos2D`)))
  (bind (_info_pos2d _info_type _info_requiredresource _info_basemovementpoints _info_movementpoints _info_path _info_pathcompleted _info_visibilitypoints _info_maintenancecost _info_state) (break `UnitInfo` (`ActorUnit.Info` (`local.ActorUnit`))))
  (bind ((`Pos2D` _pos2d) (`MapPos2D` _mappos2d)) (break `TileInfo` _value))
  (if _returnvalue
    (bind _unit (`self.SpawnUnit` null (`.Unit` (break `ProductionElement` Unit)) _pos2d _mappos2d))
    (set `local.ActorUnit` _unit)
    (bind _returnvalue_2 (`LibraryDataTables.GetUnitDataFromType` "/Game/Blueprints/Core/Data/DT_Unit.DT_Unit" _unit_unittype))
    (bind _output_get (set `local.UnitInfo` _returnvalue_2))
    (bind ((`Type` _type) (`RequiredResource` _requiredresource) (`MovementPoints` _movementpoints) (`VisibilityPoints` _visibilitypoints) (`MaintenanceCost` _maintenancecost) (`HealthPoints` _healthpoints) (`Stats` _stats)) (break `UnitData` _output_get))
    (set `ActorUnit.Info` (make `UnitInfo` (`local.Pos2D`) _type (struct) _movementpoints _movementpoints _info_path _info_pathcompleted _visibilitypoints _maintenancecost _info_state) (`local.ActorUnit`))
    (set `ActorDamageableElement.DamageableInfo` (make `DamageableInfo` (`PawnFaction.Index` (`local.Faction`)) _healthpoints _healthpoints _stats _stats) (`local.ActorUnit`))
    (`PawnFaction.AddUnit` (`local.Faction`) (`local.ActorUnit`))))

(fn `OnSettlementCreated`
  (params (Pos2D :type "IntPoint Structure (by ref)"))
  (locals (Faction :type "PawnFaction Object Reference"))
  (bind (_value _returnvalue) (`BlueprintMapLibrary.Map_Find` (`self.TilesInfo`) (`local.Pos2D`)))
  (bind (_pos2d _mappos2d) (break `TileInfo` _value))
  (if _returnvalue
    (bind _asbp_smain (cast `/Game/Blueprints/MainMode/Core/BP_SMain` (`GameplayStatics.GetGameState`)))
    (bind _currentfaction (`SMain.CurrentFaction` _asbp_smain))
    (`/Engine/EditorBlueprintResources/StandardMacros.IsValid` _currentfaction
      (:`Is Valid`
        (bind _output_get (set `local.Faction` _currentfaction))
        (bind _settlement (`self.SpawnSettlement` _output_get _pos2d _mappos2d))
        (bind _asbp_smain_2 (cast `/Game/Blueprints/MainMode/Core/BP_SMain` (`GameplayStatics.GetGameState`)))
        (bind _currentfaction_2 (`SMain.CurrentFaction` _asbp_smain_2))
        (`/Engine/EditorBlueprintResources/StandardMacros.IsValid` _currentfaction_2
          (:`Is Valid`
            (`ActorDamageableElement.SetFactionOwner` _settlement (`PawnFaction.Index` _currentfaction_2))
            (`PawnFaction.AddSettlement` _currentfaction_2 _settlement)))))))

(fn `OnUnitDestroyed`
  (params (Unit :type "ActorUnit Object Reference"))
  (locals (UnitPos :type "IntPoint Structure"))
  (`/Engine/EditorBlueprintResources/StandardMacros.IsValid` Unit
    (:`Is Valid`
      (bind _asbp_smain (cast `/Game/Blueprints/MainMode/Core/BP_SMain` (`GameplayStatics.GetGameState`)))
      (bind _currentfaction (`SMain.CurrentFaction` _asbp_smain))
      (`/Engine/EditorBlueprintResources/StandardMacros.IsValid` _currentfaction
        (:`Is Valid`
          (`PawnFaction.RemoveUnit` _currentfaction (`local.Unit`))
          (set `local.UnitPos` (`ActorUnit.GetPos` (`local.Unit`)))
          (`self.K2_DestroyActor` (`local.Unit`)) ; Se destruye la unidad
          (`self.RemoveUnitFromTile` (`local.UnitPos`))
          ;[0 0 0] Se deselecciona la casilla
          (bind _asbp_cmain (cast `/Game/Blueprints/MainMode/Core/BP_CMain` (`GameplayStatics.GetPlayerController` 0)))
          (`/Game/Blueprints/MainMode/Core/BP_CMain.UnselectTile` _asbp_cmain))))))

(fn `OnUnitProduced`
  (params (Pos2D :type "IntPoint Structure (by ref)") (Unit :type "ProductionElement Structure (by ref)"))
  (locals (UnitInfo :type "UnitData Structure") (ActorUnit :type "ActorUnit Object Reference"))
  (bind _asbp_smain (cast `/Game/Blueprints/MainMode/Core/BP_SMain` (`GameplayStatics.GetGameState`)))
  (bind _currentfaction (`SMain.CurrentFaction` _asbp_smain))
  (`/Engine/EditorBlueprintResources/StandardMacros.IsValid` _currentfaction
    (:`Is Valid`
      (`self.InitUnit` _currentfaction (`local.Pos2D`) (`local.Unit`)))))

(fn `RemoveStateFromTile`
  (params (CurrTile :type "ActorTile Object Reference (by ref)") (TileStates :type "Array of ETileState Enum"))
  (for _array_element TileStates
    ;[0 0 0] Se obtienen las casillas con el estado dado y se elimina la actual
    (bind _returnvalue (`self.GetTilesWithState` _array_element))
    (`KismetArrayLibrary.Array_RemoveItem` _returnvalue (`ActorTile.GetPos` (`local.CurrTile`)))
    (`BlueprintMapLibrary.Map_Add` (`self.TilesWithState`) _array_element (make `TilesArray` _returnvalue)))
  (`ActorTile.RemoveState` (`local.CurrTile`) (`local.TileStates`))
  (`self.UpdateTileVisual` (`local.CurrTile`)))

(fn `SpawnSettlement`
  (params (Faction :type "PawnFaction Object Reference") (Pos2D :type "IntPoint Structure (by ref)") (MapPos2D :type "Vector2D Structure"))
  (returns (Settlement :type "ActorSettlement Object Reference"))
  (locals (NewSettlement :type "/Game/Blueprints/MainMode/GameElements/BP_Settlement Object Reference"))
  (bind (_mappos2d_x _mappos2d_y) (`KismetMathLibrary.BreakVector2D` (`local.MapPos2D`)))
  (bind _newsettlement (`local.NewSettlement`))
  (if (`LibraryTileMap.CheckValidPosition` Pos2D (make `IntPoint` (`self.Rows`) (`self.Cols`)))
    (bind _returnvalue (`|SpawnActorFromClass` "/Game/Blueprints/MainMode/GameElements/BP_Settlement.BP_Settlement_C" (`KismetMathLibrary.MakeTransform` (`KismetMathLibrary.MakeVector` _mappos2d_x _mappos2d_y)) "AlwaysSpawn" "OverrideRootScale" null null)) ; Se crea el actor
    (bind _output_get (set `local.NewSettlement` _returnvalue))
    (`ActorSettlement.SetPos` _output_get (`local.Pos2D`)) ; Se establece la posicion
    (`self.AddSettlementToTile` (`local.Pos2D`) (`local.NewSettlement`)) ; Se anade a la casilla
    (`ActorSettlement.SetInitialOwnedTiles` (`local.NewSettlement`)) ; Se establecen las casillas iniciales
    ;[0 0 0] Se crean las asociaciones con los diferentes eventos
    (add `ActorSettlement.OnSettlementStateChanged` _newsettlement (`|CreateDelegate` (`local.Faction`) :!event `OnSettlementStateUpdated`))
    (add `ActorSettlement.OnUnitProduced` _newsettlement (`|CreateDelegate` :!event `OnUnitProduced`))
    (return (`local.NewSettlement`))))

(fn `SpawnUnit`
  (params (Faction :type "PawnFaction Object Reference") (Class :type "Actor Class Reference") (Pos2D :type "IntPoint Structure (by ref)") (MapPos2D :type "Vector2D Structure"))
  (returns (Unit :type "ActorUnit Object Reference"))
  (locals (NewUnit :type "ActorUnit Object Reference"))
  (bind (_mappos2d_x _mappos2d_y) (`KismetMathLibrary.BreakVector2D` (`local.MapPos2D`)))
  (if (`LibraryTileMap.CheckValidPosition` Pos2D (make `IntPoint` (`self.Rows`) (`self.Cols`)))
    (bind _returnvalue (`|SpawnActorFromClass` (`local.Class`) (`KismetMathLibrary.MakeTransform` (`KismetMathLibrary.MakeVector` _mappos2d_x _mappos2d_y)) "AlwaysSpawn" "OverrideRootScale" null null)) ; Se crea el actor
    (bind _asactor_unit (cast `ActorUnit` _returnvalue))
    (bind _output_get (set `local.NewUnit` _asactor_unit))
    (`ActorUnit.SetPos` _output_get (`local.Pos2D`)) ; Se establece su posicion
    (`self.AddUnitToTile` (`local.Pos2D`) _asactor_unit) ; Se anade la referencia a la casilla
    ;[0 0 0] Se crean las asociaciones a los diferentes eventos
    (add `ActorUnit.OnUnitDestroyed` (`local.NewUnit`) (`|CreateDelegate` :!event `OnUnitDestroyed`))
    (bind _asbp_civil_unit (cast `/Game/Blueprints/MainMode/GameElements/Units/BP_CivilUnit` (`local.NewUnit`))
      (:`then`
        (add `ActorCivilUnit.OnResourceGathered` _asbp_civil_unit (`|CreateDelegate` :!event `GatherResource`))
        (add `ActorCivilUnit.OnSettlementCreated` _asbp_civil_unit (`|CreateDelegate` :!event `OnSettlementCreated`)))
      (:`CastFailed`
        _))
    (add `ActorUnit.OnUnitStateChanged` (`local.NewUnit`) (`|CreateDelegate` (`local.Faction`) :!event `OnUnitStateUpdated`))
    (return (`local.NewUnit`))))

(fn `UpdateSelectedTile`
  (params (TileType :type "ETileType Enum" :default "None"))
  (locals (PlayerController :type "CBase Object Reference") (TileInfo :type "TileInfo Structure"))
  (bind _tileinfo_pos2d (break `TileInfo` (`local.TileInfo`)))
  (bind (_tileinfo_pos2d_2 _tileinfo_mappos2d _tileinfo_owner _tileinfo_type _tileinfo_elements _tileinfo_states) (break `TileInfo` (`local.TileInfo`)))
  (bind _tileinfo_pos2d_3 (break `TileInfo` (`local.TileInfo`)))
  (bind _ascbase (cast `CBase` (`GameplayStatics.GetPlayerController` 0)))
  (set `local.PlayerController` _ascbase)
  (bind (_value _returnvalue) (`BlueprintMapLibrary.Map_Find` (`self.TilesInfo`) (`ActorTile.GetPos` (`CBase.SelectedTile` _ascbase))))
  (if _returnvalue
    (set `local.TileInfo` _value))
  (`self.UpdateTileAtPos` _tileinfo_pos2d (`local.TileType`))
  (`self.DisplayTile` (make `TileInfo` _tileinfo_pos2d_2 _tileinfo_mappos2d -1 (`local.TileType`) _tileinfo_elements _tileinfo_states))
  (bind _asbp_ceditor (cast `/Game/Blueprints/EditorMode/Core/BP_CEditor` (`GameplayStatics.GetPlayerController` 0)))
  (`/Game/Blueprints/EditorMode/Core/BP_CEditor.UpdateSelectedTile` _asbp_ceditor _tileinfo_pos2d_3))

(fn `UpdateTileVisual`
  (params (CurrTile :type "ActorTile Object Reference (by ref)"))
  (bind (_info_pos2d _info_mappos2d _info_owner _info_type _info_elements _info_states) (break `TileInfo` (`ActorTile.Info` (`local.CurrTile`))))
  (`/Engine/EditorBlueprintResources/StandardMacros.IsValid` CurrTile
    (:`Is Valid`
      (`/Game/Blueprints/Core/GameElements/TileMap/BP_TileMapVisual.UpdateVisual` (`self.Visual`) (make `TileInfo` _info_pos2d _info_mappos2d -1 _info_type _info_elements _info_states)))))

(fn `UserConstructionScript`
  (set `self.Visual` (cast `/Game/Blueprints/Core/GameElements/TileMap/BP_TileMapVisual` (`ChildActorComponent.ChildActor` (`self.ChildActor_Visual`)) :!pure true)))