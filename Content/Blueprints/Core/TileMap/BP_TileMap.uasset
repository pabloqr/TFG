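; Hex tile map actor that generates the world from the game instance's temperature and sea level settings on BeginPlay.
; It sizes the grid from the hex mesh bounds, places a tile Blueprint per terrain type and forwards changes to a child-actor visual.
; It indexes tile states for bulk clearing and supports editing the selected tile.
; It also spawns units and settlements, links them to tiles and registers produced ones with the player faction.
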(event `self.ReceiveBeginPlay`
  (`self.SetActorTickEnabled` false)
  (`self.CalculateTileSize` "/Game/Assets/Models/HexTile.HexTile")
  (bind _asbp_ginstance (cast `/Game/Blueprints/Core/BP_GInstance` (`GameplayStatics.GetGameInstance`)))
  (`self.GenerateMap` (`GInstance.MapTemperature` _asbp_ginstance) (`GInstance.MapSeaLevel` _asbp_ginstance))
  (`/Game/Blueprints/Core/TileMap/BP_TileMapVisual.InitVisual` (`self.Visual`) self)
  (`self.DisplayMap`))

(event `self.ReceiveTick`
  (params (DeltaSeconds :type "Float (single-precision)")))

(fn `AddStateToTile`
  (params (CurrTile :type "ActorTile Object Reference (by ref)") (TileStates :type "Array of ETileState Enum"))
  (for _array_element TileStates
    ;[0 0 0] Se obtienen las casillas con el estado dado y se anade la actual a la lista
    (bind _returnvalue (`self.GetTilesWithState` _array_element))
    (`KismetArrayLibrary.Array_Add` _returnvalue (`ActorTile.GetPos` (`local.CurrTile`)))
    (`BlueprintMapLibrary.Map_Add` (`self.TilesWithState`) _array_element (make `TilesArray` _returnvalue)))
  (`ActorTile.AddState` (`local.CurrTile`) (`local.TileStates`))
  (`self.UpdateTileVisual` (`local.CurrTile`)))

(fn `CalculateTileSize`
  (params (DefaultMesh :type "StaticMesh Object Reference"))
  (bind _returnvalue (`StaticMesh.GetBoundingBox` DefaultMesh))
  (bind _returnvalue_2 (* (.x (`.Max` (break `Box` _returnvalue))) (`KismetMathLibrary.Sqrt` 3.0)))
  (set `self.TileSize` (`KismetMathLibrary.MakeVector2D` (.x (`.Max` (break `Box` _returnvalue))) (.y (`.Max` (break `Box` _returnvalue)))))
  (set `self.HorizontalOffset` (+ (.x (`.Max` (break `Box` _returnvalue))) (/ (.x (`.Max` (break `Box` _returnvalue))) 2.0)))
  (set `self.VerticalOffset` _returnvalue_2)
  (set `self.RowOffset` (/ _returnvalue_2 2.0)))

(fn `ClearStateFromTiles`
  (params (State :type "ETileState Enum" :default "None"))
  (bind _returnvalue (`self.GetTilesWithState` State))
  (`BlueprintMapLibrary.Map_Remove` (`self.TilesWithState`) (`local.State`))
  (for _array_element _returnvalue
    (bind _returnvalue_2 (`self.GetTileAtPos` _array_element))
    (`/Engine/EditorBlueprintResources/StandardMacros.IsValid` _returnvalue_2
      (:`Is Valid`
        (`self.RemoveStateFromTile` _returnvalue_2 (`|MakeArray` (`local.State`)))))))

(fn `DisplayMap`
  (bind _values (`BlueprintMapLibrary.Map_Values` (`self.TilesInfo`)))
  (for _array_element _values
    (`self.DisplayTile` _array_element)))

(fn `DisplayTile`
  (params (Info :type "TileInfo Structure"))
  (bind (_pos2d _mappos2d _type) (break `TileInfo` Info))
  (bind (_info_pos2d _info_mappos2d _info_type _info_elements) (break `TileInfo` (`local.Info`)))
  (if (`|EnumInequality` _type)
    (`self.DisplayTileAtPos` (select `ETileType` _type :`Plains` "/Game/Blueprints/MainMode/GameElements/Tiles/BP_Tile_Plains.BP_Tile_Plains_C" :`Hills` "/Game/Blueprints/MainMode/GameElements/Tiles/BP_Tile_Hills.BP_Tile_Hills_C" :`Forest` "/Game/Blueprints/MainMode/GameElements/Tiles/BP_Tile_Forest.BP_Tile_Forest_C" :`SnowPlains` "/Game/Blueprints/MainMode/GameElements/Tiles/BP_Tile_Snow.BP_Tile_Snow_C" :`SnowHills` "/Game/Blueprints/MainMode/GameElements/Tiles/BP_Tile_Snow.BP_Tile_Snow_C" :`Ice` "/Game/Blueprints/MainMode/GameElements/Tiles/BP_Tile_Ice.BP_Tile_Ice_C" :`Mountains` "/Game/Blueprints/MainMode/GameElements/Tiles/BP_Tile_Mountains.BP_Tile_Mountains_C" :`Water` "/Game/Blueprints/MainMode/GameElements/Tiles/BP_Tile_Water.BP_Tile_Water_C" :!type "ActorTile Class Reference") (`local.Info`))
    (`/Game/Blueprints/Core/TileMap/BP_TileMapVisual.UpdateVisual` (`self.Visual`) (make `TileInfo` _info_pos2d _info_mappos2d _info_type _info_elements (`|MakeArray` "None" :!type "ETileState Enum")))))

(fn `GetTileUnderCursor`
  (returns (Tile :type "/Game/Blueprints/MainMode/GameElements/Tiles/BP_Tile Object Reference"))
  (bind _ascbase (cast `CBase` (`GameplayStatics.GetPlayerController` 0)))
  (bind (_hitresult _returnvalue) (`PlayerController.GetHitResultUnderCursorByChannel` _ascbase "TraceTypeQuery3" true))
  (if _returnvalue
    (bind _asbp_tile (cast `/Game/Blueprints/MainMode/GameElements/Tiles/BP_Tile` (`.HitActor` (`GameplayStatics.BreakHitResult` _hitresult))))
    (return _asbp_tile)
    (else
      (return null))))

(fn `OnSettlementCreated`
  (params (Pos2D :type "IntPoint Structure (by ref)"))
  (bind (_value _returnvalue) (`BlueprintMapLibrary.Map_Find` (`self.TilesInfo`) (`local.Pos2D`)))
  (bind (_pos2d _mappos2d) (break `TileInfo` _value))
  (if _returnvalue
    (bind _settlement (`self.SpawnSettlement` _pos2d _mappos2d))
    (bind _asbp_settlement (cast `/Game/Blueprints/MainMode/GameElements/BP_Settlement` _settlement))
    (bind _asbp_pfaction (cast `/Game/Blueprints/MainMode/Core/BP_PFaction` (`GameplayStatics.GetPlayerPawn` 0)))
    (`KismetArrayLibrary.Array_AddUnique` (`PawnFaction.Settlements` _asbp_pfaction) _asbp_settlement)))

(fn `OnUnitProduced`
  (params (Pos2D :type "IntPoint Structure (by ref)") (Unit :type "ActorUnit Class Reference"))
  (bind _unit (`local.Unit`))
  (bind (_value _returnvalue) (`BlueprintMapLibrary.Map_Find` (`self.TilesInfo`) (`local.Pos2D`)))
  (bind (_pos2d _mappos2d) (break `TileInfo` _value))
  (if _returnvalue
    (bind _unit_2 (`self.SpawnUnit` (`local.Unit`) _pos2d _mappos2d))
    (if (== _unit "/Game/Blueprints/MainMode/GameElements/Units/BP_MilitaryUnit.BP_MilitaryUnit_C")
      (bind _asbp_military_unit (cast `/Game/Blueprints/MainMode/GameElements/Units/BP_MilitaryUnit` _unit_2))
      (bind _asbp_pfaction (cast `/Game/Blueprints/MainMode/Core/BP_PFaction` (`GameplayStatics.GetPlayerPawn` 0)))
      (`KismetArrayLibrary.Array_AddUnique` (`PawnFaction.Units` _asbp_pfaction) _asbp_military_unit)
      (elif (== _unit "/Game/Blueprints/MainMode/GameElements/Units/BP_CivilUnit.BP_CivilUnit_C")
        (bind _asbp_civil_unit (cast `/Game/Blueprints/MainMode/GameElements/Units/BP_CivilUnit` _unit_2))
        (bind _asbp_pfaction_2 (cast `/Game/Blueprints/MainMode/Core/BP_PFaction` (`GameplayStatics.GetPlayerPawn` 0)))
        (`KismetArrayLibrary.Array_AddUnique` (`PawnFaction.Units` _asbp_pfaction_2) _asbp_civil_unit)))))

(fn `RemoveStateFromTile`
  (params (CurrTile :type "ActorTile Object Reference (by ref)") (TileStates :type "Array of ETileState Enum"))
  (for _array_element TileStates
    ;[0 0 0] Se obtienen las casillas con el estado dado y se elimina la actual
    (bind _returnvalue (`self.GetTilesWithState` _array_element))
    (`KismetArrayLibrary.Array_RemoveItem` _returnvalue (`ActorTile.GetPos` (`local.CurrTile`)))
    (`BlueprintMapLibrary.Map_Add` (`self.TilesWithState`) _array_element (make `TilesArray` _returnvalue)))
  (`ActorTile.RemoveState` (`local.CurrTile`) (`local.TileStates`))
  (`self.UpdateTileVisual` (`local.CurrTile`)))

(fn `SpawnSettlement`
  (params (Pos2D :type "IntPoint Structure (by ref)") (MapPos2D :type "Vector2D Structure"))
  (returns (Settlement :type "Actor Object Reference"))
  (locals (NewSettlement :type "/Game/Blueprints/MainMode/GameElements/BP_Settlement Object Reference"))
  (bind _pos2d (`local.Pos2D`))
  (bind (_mappos2d_x _mappos2d_y) (`KismetMathLibrary.BreakVector2D` (`local.MapPos2D`)))
  (bind _newsettlement (`local.NewSettlement`))
  (bind _returnvalue (`self.GetPositionInArray` _pos2d))
  (bind _output (`|GetArrayItem` (`self.Tiles`) _returnvalue))
  (bind _info (`ActorTile.Info` _output))
  (if (`LibraryTileMap.CheckValidPosition` Pos2D (make `IntPoint` (`self.Rows`) (`self.Cols`)))
    (bind _returnvalue_2 (`|SpawnActorFromClass` "/Game/Blueprints/MainMode/GameElements/BP_Settlement.BP_Settlement_C" (`KismetMathLibrary.MakeTransform` (`KismetMathLibrary.MakeVector` _mappos2d_x _mappos2d_y)) "AlwaysSpawn" "OverrideRootScale" null null))
    (bind _output_get (set `local.NewSettlement` _returnvalue_2))
    (`ActorSettlement.SetPos` _output_get _pos2d)
    (if (!= _returnvalue -1)
      (set `ActorTile.Info` (make `TileInfo` (break `TileInfo` _info) (`.MapPos2D` (break `TileInfo` _info)) (`.Type` (break `TileInfo` _info)) (make `TileElements` (break `TileElements` (`.Elements` (break `TileInfo` _info))) (`.Unit` (break `TileElements` (`.Elements` (break `TileInfo` _info)))) (`local.NewSettlement`)) (`.States` (break `TileInfo` _info))) _output)
      (`ActorSettlement.SetInitialOwnedTiles` (`local.NewSettlement`))
      (bind _aspawn_faction (cast `PawnFaction` (`GameplayStatics.GetPlayerPawn` 0))
        (:`then`
          (add `ActorSettlement.OnSettlementStateChanged` _newsettlement (`|CreateDelegate` _aspawn_faction :!event `OnSettlementStateUpdated`))
          (add `ActorSettlement.OnUnitProduced` _newsettlement (`|CreateDelegate` :!event `OnUnitProduced`)))
        (:`CastFailed`
          _))
      (return (`local.NewSettlement`)))))

(fn `SpawnUnit`
  (params (Class :type "Actor Class Reference") (Pos2D :type "IntPoint Structure (by ref)") (MapPos2D :type "Vector2D Structure"))
  (returns (Unit :type "Actor Object Reference"))
  (locals (NewUnit :type "Actor Object Reference"))
  (bind (_mappos2d_x _mappos2d_y) (`KismetMathLibrary.BreakVector2D` (`local.MapPos2D`)))
  (bind _pos2d (`local.Pos2D`))
  (bind _returnvalue (`self.GetPositionInArray` _pos2d))
  (bind _output (`|GetArrayItem` (`self.Tiles`) _returnvalue))
  (bind _info (`ActorTile.Info` _output))
  (if (`LibraryTileMap.CheckValidPosition` Pos2D (make `IntPoint` (`self.Rows`) (`self.Cols`)))
    (bind _returnvalue_2 (`|SpawnActorFromClass` (`local.Class`) (`KismetMathLibrary.MakeTransform` (`KismetMathLibrary.MakeVector` _mappos2d_x _mappos2d_y)) "AlwaysSpawn" "OverrideRootScale" null null))
    (bind _output_get (set `local.NewUnit` _returnvalue_2))
    (bind _asactor_unit (cast `ActorUnit` _output_get))
    (`ActorUnit.SetPos` _asactor_unit _pos2d)
    (if (!= _returnvalue -1)
      (set `ActorTile.Info` (make `TileInfo` (break `TileInfo` _info) (`.MapPos2D` (break `TileInfo` _info)) (`.Type` (break `TileInfo` _info)) (make `TileElements` (break `TileElements` (`.Elements` (break `TileInfo` _info))) _asactor_unit (`.Settlement` (break `TileElements` (`.Elements` (break `TileInfo` _info))))) (`.States` (break `TileInfo` _info))) _output)
      (bind _aspawn_faction (cast `PawnFaction` (`GameplayStatics.GetPlayerPawn` 0))
        (:`then`
          (add `ActorUnit.OnUnitStateChanged` _asactor_unit (`|CreateDelegate` _aspawn_faction :!event `OnUnitStateUpdated`)))
        (:`CastFailed`
          _))
      (return (`local.NewUnit`)))))

(fn `UpdateSelectedTile`
  (params (TileType :type "ETileType Enum" :default "None"))
  (locals (PlayerController :type "CBase Object Reference") (TileInfo :type "TileInfo Structure"))
  (bind _tileinfo_pos2d (break `TileInfo` (`local.TileInfo`)))
  (bind (_tileinfo_pos2d_2 _tileinfo_mappos2d _tileinfo_type _tileinfo_elements _tileinfo_states) (break `TileInfo` (`local.TileInfo`)))
  (bind _tileinfo_pos2d_3 (break `TileInfo` (`local.TileInfo`)))
  (bind _ascbase (cast `CBase` (`GameplayStatics.GetPlayerController` 0)))
  (set `local.PlayerController` _ascbase)
  (bind (_value _returnvalue) (`BlueprintMapLibrary.Map_Find` (`self.TilesInfo`) (`ActorTile.GetPos` (`CBase.SelectedTile` _ascbase))))
  (if _returnvalue
    (set `local.TileInfo` _value))
  (`self.UpdateTileAtPos` _tileinfo_pos2d (`local.TileType`))
  (`self.DisplayTile` (make `TileInfo` _tileinfo_pos2d_2 _tileinfo_mappos2d (`local.TileType`) _tileinfo_elements _tileinfo_states))
  (bind _asbp_ceditor (cast `/Game/Blueprints/EditorMode/Core/BP_CEditor` (`GameplayStatics.GetPlayerController` 0)))
  (`/Game/Blueprints/EditorMode/Core/BP_CEditor.UpdateSelectedTile` _asbp_ceditor _tileinfo_pos2d_3))

(fn `UpdateTileVisual`
  (params (CurrTile :type "ActorTile Object Reference (by ref)"))
  (bind (_info_pos2d _info_mappos2d _info_type _info_elements _info_states) (break `TileInfo` (`ActorTile.Info` (`local.CurrTile`))))
  (`/Engine/EditorBlueprintResources/StandardMacros.IsValid` CurrTile
    (:`Is Valid`
      (`/Game/Blueprints/Core/TileMap/BP_TileMapVisual.UpdateVisual` (`self.Visual`) (make `TileInfo` _info_pos2d _info_mappos2d _info_type _info_elements _info_states)))))

(fn `UserConstructionScript`
  (set `self.Visual` (cast `/Game/Blueprints/Core/TileMap/BP_TileMapVisual` (`ChildActorComponent.ChildActor` (`self.ChildActor_Visual`)) :!pure true)))