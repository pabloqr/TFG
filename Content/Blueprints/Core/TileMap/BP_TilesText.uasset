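; Tile map text overlay actor that labels accessible tiles on the selected unit's path with their total turn count.
; On BeginPlay it binds to BP_TileMap's tile-info and path events.
; It lazily spawns TextRenderActors cached in a map by grid position, destroying them for inaccessible tiles or when the overlay is hidden.
; TilesInPath tracks labeled path tiles so they can be refreshed when the path is reset.
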(event `self.ReceiveBeginPlay`
  (bind _returnvalue (`GameplayStatics.GetActorOfClass` "/Game/Blueprints/Core/TileMap/BP_TileMap.BP_TileMap_C"))
  (bind _output_get (set `self.TileMap` _returnvalue))
  (add `ActorTileMap.OnTileInfoUpdated` _output_get (`|CreateDelegate` :!event `UpdateTextOnTile`))
  (add `ActorTileMap.OnPathCreated` (`self.TileMap`) (`|CreateDelegate` :!event `ResetTilesText`))
  (add `ActorTileMap.OnPathUpdated` (`self.TileMap`) (`|CreateDelegate` :!event `UpdateTextOnTileFromPath`)))

(fn `ClearTextActors`
  (bind _values (`BlueprintMapLibrary.Map_Values` (`self.TilesText`)))
  (for _array_element _values
    (`self.K2_DestroyActor` _array_element))
  (`BlueprintMapLibrary.Map_Clear` (`self.TilesText`)))

(fn `DestroyTextActor`
  (params (Pos2D :type "IntPoint Structure"))
  (locals (Actor :type "TextRenderActor Object Reference"))
  (bind _output_get (set `local.Actor` (`BlueprintMapLibrary.Map_Find` (`self.TilesText`) Pos2D)))
  (`/Engine/EditorBlueprintResources/StandardMacros.IsValid` _output_get
    (:`Is Valid`
      (`self.K2_DestroyActor` (`local.Actor`))
      (`BlueprintMapLibrary.Map_Remove` (`self.TilesText`) (`local.Pos2D`)))))

(fn `GetTextActor`
  (params (Pos2D :type "IntPoint Structure"))
  (returns (TextActor :type "TextRenderActor Object Reference"))
  (locals (Actor :type "TextRenderActor Object Reference"))
  (bind _actor (`local.Actor`))
  (bind _textrender (`TextRenderActor.TextRender` (`local.Actor`)))
  (bind _output_get (set `local.Actor` (`BlueprintMapLibrary.Map_Find` (`self.TilesText`) Pos2D)))
  (`/Engine/EditorBlueprintResources/StandardMacros.IsValid` _output_get
    (:`Is Valid`
      (return (`local.Actor`)))
    (:`Is Not Valid`
      ;[0 0 0] Si no se encuentra el actor, se crea y se anade al diccionario de actores
      (bind _returnvalue (`|SpawnActorFromClass` "/Script/Engine.TextRenderActor" (`KismetMathLibrary.MakeTransform` (0.0 0.0 0.0)) "AlwaysSpawn" "OverrideRootScale" null null))
      (bind _output_get_2 (set `local.Actor` _returnvalue))
      (`BlueprintMapLibrary.Map_Add` (`self.TilesText`) (`local.Pos2D`) _output_get_2)
      ;[0 0 0] Se desactiva el metodo tick y las colisiones del actor
      (`self.SetActorTickEnabled` _actor false)
      (`self.SetActorEnableCollision` _actor false)
      ;[0 0 0] Se centra el texto
      (`TextRenderComponent.SetHorizontalAlignment` _textrender "EHTA_Center")
      (`TextRenderComponent.SetVerticalAlignment` _textrender "EVRTA_TextCenter")
      (`TextRenderComponent.SetTextRenderColor` _textrender (make `Color` 0 0 0 1))
      (return (`local.Actor`)))))

(fn `GetTextFromPath`
  (params (Path :type "Array of Movement Structure") (Pos2D :type "IntPoint Structure") (UnitBaseMovementPoints :type Integer) (UnitMovementPoints :type Integer) (UnitState :type "EUnitState Enum" :default "None"))
  (returns (Text :type String))
  (locals (PathInfo :type "Movement Structure"))
  (bind _returnvalue (`LibraryTileMap.IsTileInPath` Path Pos2D))
  (if (!= _returnvalue -1)
    (bind _output_get (set `local.PathInfo` (`|GetArrayItem` Path _returnvalue)))
    (`BlueprintSetLibrary.Set_Add` (`self.TilesInPath`) (`local.Pos2D`))
    (return (`KismetStringLibrary.Conv_IntToString` (`.TotalTurns` (break `Movement` _output_get))))
    (else
      (return ""))))

(fn `ResetTilesText`
  (params (Tiles :type "Array of Movement Structure"))
  (locals (TmpTilesInPath :type "Set of IntPoint Structure"))
  (bind _tilesinpath (`self.TilesInPath`))
  (if (== (`KismetArrayLibrary.Array_Length` Tiles) 0)
    (bind _result (`BlueprintSetLibrary.Set_ToArray` _tilesinpath))
    (`BlueprintSetLibrary.Set_Clear` _tilesinpath)
    (for _array_element _result
      (`self.UpdateTextOnTileFromPath` _array_element (`|MakeArray`)))
    (else
      (set `local.TmpTilesInPath` (`self.TilesInPath`))
      (`BlueprintSetLibrary.Set_Clear` (`self.TilesInPath`))
      (for _array_element_2 (`local.Tiles`)
        (bind _pos2d (break `Movement` _array_element_2))
        (if (not (`BlueprintSetLibrary.Set_Contains` (`local.TmpTilesInPath`) _pos2d))
          (`self.UpdateTextOnTileFromPath` _pos2d (`local.Tiles`)))))))

(fn `SetShowTilesInfo`
  (params (ShowTilesInfo :type Boolean))
  (bind _output_get (set `self.ShowTilesInfo` ShowTilesInfo))
  (if _output_get
    (bind _keys (`BlueprintMapLibrary.Map_Keys` (`ActorTileMap.TilesInfo` (`self.TileMap`))))
    (for _array_element _keys
      (`self.UpdateTextOnTileFromPath` _array_element (`|MakeArray`)))
    (else
      (`self.ClearTextActors`)
      (`BlueprintSetLibrary.Set_Clear` (`self.TilesInPath`)))))

(fn `UpdateTextOnTile`
  (params (Pos2D :type "IntPoint Structure"))
  (`self.UpdateTextOnTileFromPath` Pos2D (`|MakeArray`)))

(fn `UpdateTextOnTileFromPath`
  (params (Pos2D :type "IntPoint Structure") (Path :type "Array of Movement Structure"))
  (locals (PlayerController :type "/Game/Blueprints/MainMode/Core/BP_CMain Object Reference") (Actor :type "TextRenderActor Object Reference") (TileInfo :type "TileInfo Structure") (TileText :type String) (PathInfo :type "Movement Structure"))
  (bind _tileinfo (`local.TileInfo`))
  (bind (_value _returnvalue) (`BlueprintMapLibrary.Map_Find` (`ActorTileMap.TilesInfo` (`self.TileMap`)) (`local.Pos2D`)))
  (bind (_info_pos2d _info_basemovementpoints _info_movementpoints _info_path _info_pathcompleted _info_visibilitypoints _info_productioncost _info_maintenancecost _info_state) (break `UnitInfo` (`ActorUnit.Info` (`CMain.Unit` (`local.PlayerController`)))))
  (if (`self.ShowTilesInfo`)
    (if _returnvalue
      (bind _output_get (set `local.TileInfo` _value))
      (if (`LibraryTileMap.IsTileTypeAccesible` (`.Type` (break `TileInfo` _output_get)))
        (`|ExecutionSequence`
          (:`then_0`
            (bind _asbp_cmain (cast `/Game/Blueprints/MainMode/Core/BP_CMain` (`GameplayStatics.GetPlayerController` 0)))
            (set `local.PlayerController` _asbp_cmain)
            (`/Engine/EditorBlueprintResources/StandardMacros.IsValid` (`CMain.Unit` (`local.PlayerController`))
              (:`Is Valid`
                (bind _assplayer_main (cast `SPlayerMain` (`Controller.PlayerState` (`local.PlayerController`))))
                (bind _text (`self.GetTextFromPath` (`local.Path`) (`local.Pos2D`) _info_basemovementpoints _info_movementpoints _info_state))
                (bind _output_get_2 (set `local.TileText` _text))
                (if (`KismetStringLibrary.IsEmpty` _output_get_2)
                  _))))
          (:`then_1`
            (bind _textactor (`self.GetTextActor` (`local.Pos2D`)))
            (set `local.Actor` _textactor)
            (`TextRenderComponent.K2_SetText` (`TextRenderActor.TextRender` (`local.Actor`)) (`KismetTextLibrary.Conv_StringToText` (`local.TileText`)))
            (`self.K2_SetActorTransform` (`local.Actor`) (`KismetMathLibrary.MakeTransform` (`KismetMathLibrary.MakeVector` (+ (`KismetMathLibrary.BreakVector2D` (`.MapPos2D` (break `TileInfo` _tileinfo))) 0.0) (`.Y` (`KismetMathLibrary.BreakVector2D` (`.MapPos2D` (break `TileInfo` _tileinfo)))) 15.0) (struct :`Pitch` 90.0 :`Yaw` 90.0) (2.0 2.0 2.0)) false false)))
        (else
          (`self.DestroyTextActor` (`local.Pos2D`) :!label _label)))
      (else
        (goto _label)))))

(fn `UserConstructionScript`)