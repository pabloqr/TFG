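; BP_HexGrid is an actor that lays out a Width by Height grid of hexagonal tiles in its construction script.
; It derives outer and inner radii from the tile mesh bounds and Scale, then spaces tiles with an adjustable gap, using a FlipFlop to stagger alternate rows.
; An Instance flag selects instanced mesh tiles or BP_HexTile child actors.
; BeginPlay prints the radii and edge length.
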(event `self.ReceiveBeginPlay`
  (`KismetSystemLibrary.PrintString` "Outter" true true (struct :`G` 0.66 :`B` 1.0 :`A` 1.0) 20.0)
  (`KismetSystemLibrary.PrintString` (`KismetStringLibrary.Conv_DoubleToString` (`self.OutterRadius`)) true true (struct :`G` 0.66 :`B` 1.0 :`A` 1.0) 20.0)
  (`KismetSystemLibrary.PrintString` "Inner" true true (struct :`G` 0.66 :`B` 1.0 :`A` 1.0) 20.0)
  (`KismetSystemLibrary.PrintString` (`KismetStringLibrary.Conv_DoubleToString` (`self.InnerRadius`)) true true (struct :`G` 0.66 :`B` 1.0 :`A` 1.0) 20.0)
  (`KismetSystemLibrary.PrintString` "Edge" true true (struct :`G` 0.66 :`B` 1.0 :`A` 1.0) 20.0)
  (`KismetSystemLibrary.PrintString` (`KismetStringLibrary.Conv_DoubleToString` (`self.EdgeLength`)) true true (struct :`G` 0.66 :`B` 1.0 :`A` 1.0) 20.0))

(fn `UserConstructionScript`
  (`StaticMeshComponent.SetStaticMesh` (`self.Grid`) (`self.TileMesh`))
  (bind _output_get (set `self.OutterRadius` (* (.x (`.Max` (break `Box` (`StaticMesh.GetBoundingBox` (`self.TileMesh`))))) (`self.Scale`))))
  (set `self.InnerRadius` (/ (* _output_get (`KismetMathLibrary.Sqrt` 3.0)) 2.0))
  ;[1 1 1] HeightLoop
  (for _index (range (`self.Height`))
    ;[1 1 1] WidthLoop
    (for _index_2 (range (`self.Width`))
      (if (`self.Instance?`)
        (bind _returnvalue (+ (* (`KismetMathLibrary.Conv_IntToDouble` _index_2) (`self.OutterRadius`) 2.0) (* _index_2 (`self.OutterRadius`)) (* _index_2 (`self.Offset`)) (`self.RowOffset`)))
        (bind _returnvalue_2 (+ (* (`self.InnerRadius`) (`KismetMathLibrary.Conv_IntToDouble` _index)) (* _index (`self.Offset`))))
        ;[1 1 1] InstancedMesh
        (`InstancedStaticMeshComponent.AddInstance` (`self.Grid`) (`KismetMathLibrary.MakeTransform` (`KismetMathLibrary.MakeVector` _returnvalue _returnvalue_2) (struct) (`KismetMathLibrary.Conv_DoubleToVector` (`self.Scale`))))
        (else
          ;[1 1 1] ChildActors
          (bind _returnvalue_3 (`AddComponent|NODE_AddChildActorComponent-0` :`RelativeTransform` (`KismetMathLibrary.MakeTransform` (`KismetMathLibrary.MakeVector` _returnvalue _returnvalue_2) (struct) (`KismetMathLibrary.Conv_DoubleToVector` (`self.Scale`)))))
          (`ChildActorComponent.SetChildActorClass` _returnvalue_3 "/Game/Blueprints/BP_HexTile.BP_HexTile_C"))))
    (`/Engine/EditorBlueprintResources/StandardMacros.FlipFlop`
      (:`A`
        (set `self.RowOffset` (* (+ (`self.OutterRadius`) (/ (`self.OutterRadius`) 2.0)) -1.0)))
      (:`B`
        (set `self.RowOffset` 0.0)))))