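; Forest tile actor that fills itself with a randomized cluster of trees when play begins.
; BeginPlay disables ticking and calls DisplayForest, which adds a random number of instances to the Trees instanced mesh component.
; Square-root radius sampling spreads them evenly by area within a disc around the component origin, each with random yaw and uniform scale.
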(event `self.ReceiveBeginPlay`
  (`parent.ReceiveBeginPlay`)
  (`self.SetActorTickEnabled` false)
  (`self.DisplayForest`))

(fn `DisplayForest`
  (bind _returnvalue (`KismetMathLibrary.RandomFloat`))
  (for _ (range (+ (`KismetMathLibrary.RandomIntegerInRange` 100 200) 1))
    (bind _output_get (set `self.Radius` (* (`KismetMathLibrary.Sqrt` _returnvalue) 80.0)))
    (bind _output_get_2 (set `self.Alpha` (* _returnvalue 2.0 (`KismetMathLibrary.GetPI`))))
    (`InstancedStaticMeshComponent.AddInstance` (`self.Trees`) (`KismetMathLibrary.MakeTransform` (`KismetMathLibrary.MakeVector` (* (`KismetMathLibrary.Cos` _output_get_2) _output_get) (* (`KismetMathLibrary.Sin` _output_get_2) _output_get)) (`KismetMathLibrary.MakeRotator` 0.0 0.0 (`KismetMathLibrary.RandomFloatInRange` 0.0 360.0)) (`KismetMathLibrary.Conv_DoubleToVector` (`KismetMathLibrary.RandomFloatInRange` 0.01 0.04))))))

(fn `UserConstructionScript`
  (`parent.UserConstructionScript`))