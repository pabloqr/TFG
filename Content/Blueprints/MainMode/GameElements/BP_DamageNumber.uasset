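; BP_DamageNumber is a short-lived actor that shows an animated damage number in the game through a widget component.
; On BeginPlay it casts the component's user widget to Display_DamageNumber and passes it its Damage and Color values to play the damage animation.
; It binds to the end of the widget's number animation and destroys itself when that finishes.
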(event `self.ReceiveBeginPlay`
  (bind _asdisplay_damage_number (cast `/Game/Blueprints/MainMode/UI/Components/Display_DamageNumber` (`WidgetComponent.GetUserWidgetObject` (`self.DamageNumber`))))
  (`UserWidget.BindToAnimationFinished` _asdisplay_damage_number (`/Game/Blueprints/MainMode/UI/Components/Display_DamageNumber.AnimationNumber` _asdisplay_damage_number) (delegate `EventOnAnimationFinished`))
  (`/Game/Blueprints/MainMode/UI/Components/Display_DamageNumber.EventPlayDamageAnimation` _asdisplay_damage_number (`self.Damage`) (make `SlateColor` (`self.Color`))))

(event `EventOnAnimationFinished`
  (`self.K2_DestroyActor`))

(fn `UserConstructionScript`)