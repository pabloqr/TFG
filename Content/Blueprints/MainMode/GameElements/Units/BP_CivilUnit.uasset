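; Civil unit on the tile map that keeps tile occupancy in sync and animates its movement between tiles.
; On BeginPlay it caches BP_TileMap and binds to OnUnitMoved, which frees the previous tile's unit slot and claims the current one before animating.
; MoveAnimation replays a timeline for each queued move, lerping location and yaw toward the next tile until the queue is empty.
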(event `self.ReceiveBeginPlay`
  (bind _returnvalue (`GameplayStatics.GetActorOfClass` "/Game/Blueprints/Core/TileMap/BP_TileMap.BP_TileMap_C"))
  (set `self.TileMap` _returnvalue)
  (add `self.OnUnitMoved` (`|CreateDelegate` :!event `EventOnUnitMoved`)))

(event `EventOnUnitMoved` :!signature `self.OnUnitMoved`
  (params (PrevPos :type "IntPoint Structure (by ref)") (Moves :type "Array of Movement Structure"))
  (if (> (`KismetArrayLibrary.Array_Length` Moves) 0)
    (set `self.CurrMoves` Moves)
    (set `self.NewTile` (`self.GetCurrentTile`))
    (`self.UpdateTiles` PrevPos) ; Se actualizan las casillas del mapa para liberar la previa y ocupar la actual
    (`self.MoveAnimation`)))

(event `MoveAnimation`
  (bind _prevtransform_location (`KismetMathLibrary.BreakTransform` (`self.PrevTransform`)))
  (bind (_prevtransform_location_2 _prevtransform_rotation) (`KismetMathLibrary.BreakTransform` (`self.PrevTransform`)))
  (bind _prevtransform_location_3 (`KismetMathLibrary.BreakTransform` (`self.PrevTransform`)))
  (bind _currmoves (`self.CurrMoves`))
  (bind (_value _returnvalue) (`BlueprintMapLibrary.Map_Find` (`ActorTileMap.TilesInfo` (`self.TileMap`)) (`.Pos2D` (break `Movement` (`|GetArrayItem` _currmoves)))))
  (bind (_returnvalue_roll _returnvalue_pitch _returnvalue_yaw) (`KismetMathLibrary.BreakRotator` (`KismetMathLibrary.FindLookAtRotation` _prevtransform_location_3 (`KismetMathLibrary.MakeVector` (`KismetMathLibrary.BreakVector2D` (`.MapPos2D` (break `TileInfo` _value))) (`.Y` (`KismetMathLibrary.BreakVector2D` (`.MapPos2D` (break `TileInfo` _value))))))))
  (if (> (`KismetArrayLibrary.Array_Length` _currmoves) 0) :!label _label
    (if _returnvalue
      (set `self.PrevTransform` (`KismetMathLibrary.MakeTransform` (`self.K2_GetActorLocation`) (`self.K2_GetActorRotation`)))
      (bind (_direction _locationalpha _rotationalpha) (`Timeline|TimelineCivilUnitMove` :!via `PlayFromStart`)
        (:`Update`
          (bind (_returnvalue_roll_2 _returnvalue_pitch_2 _returnvalue_yaw_2) (`KismetMathLibrary.BreakRotator` (`KismetMathLibrary.RLerp` _prevtransform_rotation (`KismetMathLibrary.MakeRotator` 0.0 0.0 _returnvalue_yaw) _rotationalpha true)))
          (`self.K2_SetActorLocationAndRotation` (`KismetMathLibrary.VLerp` _prevtransform_location (`KismetMathLibrary.MakeVector` (`KismetMathLibrary.BreakVector2D` (`.MapPos2D` (break `TileInfo` _value))) (`.Y` (`KismetMathLibrary.BreakVector2D` (`.MapPos2D` (break `TileInfo` _value))))) _locationalpha) (`KismetMathLibrary.MakeRotator` 0.0 0.0 _returnvalue_yaw_2)))
        (:`Finished`
          (`KismetArrayLibrary.Array_Remove` (`self.CurrMoves`))
          (goto _label))))))

(fn `GetCurrentTile`
  (returns (Output :type "ActorTile Object Reference"))
  (bind _tilemap (`self.TileMap`))
  (return (`|GetArrayItem` (`ActorTileMap.Tiles` _tilemap) (`ActorTileMap.GetPositionInArray` _tilemap (`self.GetPos`)))))

(fn `UpdateTiles`
  (params (Pos2D :type "IntPoint Structure (by ref)"))
  (bind _newtile (`self.NewTile`))
  (bind _tilemap (`self.TileMap`))
  (bind _info (`ActorTile.Info` _newtile))
  (bind _output (`|GetArrayItem` (`ActorTileMap.Tiles` _tilemap) (`ActorTileMap.GetPositionInArray` _tilemap Pos2D)))
  (bind _info_2 (`ActorTile.Info` _output))
  (set `ActorTile.Info` (make `TileInfo` (break `TileInfo` _info_2) (`.MapPos2D` (break `TileInfo` _info_2)) (`.Type` (break `TileInfo` _info_2)) (make `TileElements` (break `TileElements` (`.Elements` (break `TileInfo` _info_2))) null (`.Settlement` (break `TileElements` (`.Elements` (break `TileInfo` _info_2))))) (`.States` (break `TileInfo` _info_2))) _output)
  (set `ActorTile.Info` (make `TileInfo` (break `TileInfo` _info) (`.MapPos2D` (break `TileInfo` _info)) (`.Type` (break `TileInfo` _info)) (make `TileElements` (break `TileElements` (`.Elements` (break `TileInfo` _info))) self (`.Settlement` (break `TileElements` (`.Elements` (break `TileInfo` _info))))) (`.States` (break `TileInfo` _info))) _newtile))

(fn `UserConstructionScript`)