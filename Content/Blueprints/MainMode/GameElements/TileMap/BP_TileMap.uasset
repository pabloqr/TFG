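; Hex tile map actor that generates the game's map on BeginPlay from the temperature and sea level stored in BP_GInstance.
; It derives hex spacing from the mesh bounds, then DisplayMap places a tile Blueprint per terrain type.
; A child-actor BP_TileMapVisual is updated for each tile and whenever tile states are added, removed or cleared.
; It also resolves the tile under the cursor by trace.
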(event `self.ReceiveBeginPlay`
  (`self.SetActorTickEnabled` false)
  (`self.CalculateTileSize` "/Game/Assets/Models/HexTile.HexTile")
  (bind _asbp_ginstance (cast `/Game/Blueprints/Core/BP_GInstance` (`GameplayStatics.GetGameInstance`)))
  (`self.GenerateMap` (`GInstance.MapTemperature` _asbp_ginstance) (`GInstance.MapSeaLevel` _asbp_ginstance))
  (`/Game/Blueprints/MainMode/GameElements/TileMap/BP_TileMapVisual.InitVisual` (`self.Visual`) self)
  (`self.DisplayMap`))

(event `self.ReceiveTick`
  (params (DeltaSeconds :type "Float (single-precision)")))

(fn `AddStateToTile`
  (params (CurrTile :type "ActorTile Object Reference (by ref)") (TileStates :type "Array of ETileState Enum"))
  (bind _currtile (`local.CurrTile`))
  (`ActorTile.AddState` CurrTile TileStates)
  (`/Game/Blueprints/MainMode/GameElements/TileMap/BP_TileMapVisual.UpdateVisual` (`self.Visual`) (make `TileInfo` (`ActorPlaceableElement.Pos2D` _currtile) (`ActorPlaceableElement.MapPos2D` _currtile) (`ActorTile.TileType` _currtile)) (`ActorTile.TileStates` _currtile)))

(fn `CalculateTileSize`
  (params (DefaultMesh :type "StaticMesh Object Reference"))
  (bind _returnvalue (`StaticMesh.GetBoundingBox` DefaultMesh))
  (bind _returnvalue_2 (* (.x (`.Max` (break `Box` _returnvalue))) (`KismetMathLibrary.Sqrt` 3.0)))
  (set `self.TileSize` (`KismetMathLibrary.MakeVector2D` (.x (`.Max` (break `Box` _returnvalue))) (.y (`.Max` (break `Box` _returnvalue)))))
  (set `self.HorizontalOffset` (+ (.x (`.Max` (break `Box` _returnvalue))) (/ (.x (`.Max` (break `Box` _returnvalue))) 2.0)))
  (set `self.VerticalOffset` _returnvalue_2)
  (set `self.RowOffset` (/ _returnvalue_2 2.0)))

(fn `ClearStateFromTiles`
  (params (State :type "ETileState Enum" :default "None"))
  (locals (TilesWithState :type "Array of IntPoint Structure"))
  (bind _output_get (set `local.TilesWithState` (`self.GetTilesWithState` State)))
  (for _array_element _output_get
    (`self.RemoveStateFromTile` (`self.GetTileAtPos` _array_element) (`|MakeArray` (`local.State`)))))

(fn `DisplayMap`
  (locals (TileInfo :type "TileInfo Structure"))
  (bind _tileinfo (`local.TileInfo`))
  (bind _tileinfo_2 (`local.TileInfo`))
  (bind _tileinfo_3 (`local.TileInfo`))
  (bind _tileinfo_4 (`local.TileInfo`))
  (for _array_element (`self.TilesInfo`)
    (set `local.TileInfo` _array_element)
    (`|ExecutionSequence`
      (:`then_0`
        (switch `ETileType` (`.TileType` (break `TileInfo` _array_element))
          (:`Plains`
            (`self.DisplayTileAtPos` "/Game/Blueprints/MainMode/GameElements/Tiles/BP_Tile_Plains.BP_Tile_Plains_C" _tileinfo_2))
          (:`Hills`
            (`self.DisplayTileAtPos` "/Game/Blueprints/MainMode/GameElements/Tiles/BP_Tile_Hills.BP_Tile_Hills_C" _tileinfo_2))
          (:`Forest`
            (`self.DisplayTileAtPos` "/Game/Blueprints/MainMode/GameElements/Tiles/BP_Tile_Forest.BP_Tile_Forest_C" _tileinfo_3))
          (:`SnowPlains`
            (`self.DisplayTileAtPos` "/Game/Blueprints/MainMode/GameElements/Tiles/BP_Tile_Snow.BP_Tile_Snow_C" _tileinfo_3))
          (:`SnowHills`
            (`self.DisplayTileAtPos` "/Game/Blueprints/MainMode/GameElements/Tiles/BP_Tile_Snow.BP_Tile_Snow_C" _tileinfo_4))
          (:`Ice`
            (`self.DisplayTileAtPos` "/Game/Blueprints/MainMode/GameElements/Tiles/BP_Tile_Ice.BP_Tile_Ice_C" _tileinfo_4))
          (:`Mountains`
            (`self.DisplayTileAtPos` "/Game/Blueprints/MainMode/GameElements/Tiles/BP_Tile_Mountains.BP_Tile_Mountains_C" _tileinfo))
          (:`Water`
            (`self.DisplayTileAtPos` "/Game/Blueprints/MainMode/GameElements/Tiles/BP_Tile_Water.BP_Tile_Water_C" _tileinfo))))
      (:`then_1`
        (`/Game/Blueprints/MainMode/GameElements/TileMap/BP_TileMapVisual.UpdateVisual` (`self.Visual`) (`local.TileInfo`) (`|MakeArray` "None" :!type "ETileState Enum"))))))

(fn `GetTileUnderCursor`
  (returns (SelectedTile :type "/Game/Blueprints/MainMode/GameElements/Tiles/BP_Tile Object Reference"))
  (locals (TileInfo :type "TileInfo Structure") (Tile :type "/Game/Blueprints/MainMode/GameElements/Tiles/BP_Tile Object Reference"))
  (bind _asbp_cmain (cast `/Game/Blueprints/MainMode/Core/BP_CMain` (`GameplayStatics.GetPlayerController` 0)))
  (bind (_hitresult _returnvalue) (`PlayerController.GetHitResultUnderCursorByChannel` _asbp_cmain "TraceTypeQuery3" true))
  (if _returnvalue
    (bind _asbp_tile (cast `/Game/Blueprints/MainMode/GameElements/Tiles/BP_Tile` (`.HitActor` (`GameplayStatics.BreakHitResult` _hitresult))))
    (set `local.Tile` _asbp_tile)
    (bind _output_get (set `local.TileInfo` (make `TileInfo` (`ActorPlaceableElement.Pos2D` _asbp_tile) (`ActorPlaceableElement.MapPos2D` _asbp_tile) (`ActorTile.TileType` _asbp_tile))))
    (return (`local.Tile`))
    (else
      (return null))))

(fn `RemoveStateFromTile`
  (params (CurrTile :type "ActorTile Object Reference") (TileStates :type "Array of ETileState Enum"))
  (bind _currtile (`local.CurrTile`))
  (`ActorTile.RemoveState` CurrTile TileStates)
  (`/Game/Blueprints/MainMode/GameElements/TileMap/BP_TileMapVisual.UpdateVisual` (`self.Visual`) (make `TileInfo` (`ActorPlaceableElement.Pos2D` _currtile) (`ActorPlaceableElement.MapPos2D` _currtile) (`ActorTile.TileType` _currtile)) (`ActorTile.TileStates` _currtile)))

(fn `UserConstructionScript`
  (set `self.Visual` (cast `/Game/Blueprints/MainMode/GameElements/TileMap/BP_TileMapVisual` (`ChildActorComponent.ChildActor` (`self.ChildActor_Visual`)) :!pure true)))