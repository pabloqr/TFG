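; Visual layer for the hex tile map, drawing tiles through a child BP_TileMapMeshInst actor.
; InitVisual stores the TileMap, sets up that actor with a flat hex mesh plus filler and border materials, and lifts itself slightly above the origin.
; UpdateVisual refreshes a tile by removing and re-adding its instance with tile states and accessibility from the TileMap.
; DesroyVisual clears all instances, and actor tick is disabled at BeginPlay.
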(event `self.ReceiveBeginPlay`
  (`self.SetActorTickEnabled` false))

(fn `DesroyVisual`
  (`/Game/Blueprints/MainMode/GameElements/TileMap/BP_TileMapMeshInst.ClearInstances` (`self.MeshInst`)))

(fn `InitVisual`
  (params (TileMap :type "/Game/Blueprints/MainMode/GameElements/TileMap/BP_TileMap Object Reference"))
  (set `self.TileMap` TileMap)
  (bind _output_get (set `self.MeshInst` (cast `/Game/Blueprints/MainMode/GameElements/TileMap/BP_TileMapMeshInst` (`ChildActorComponent.ChildActor` (`self.ChildActor_MeshInst`)) :!pure true)))
  (`/Game/Blueprints/MainMode/GameElements/TileMap/BP_TileMapMeshInst.InitMeshInst` :`self` _output_get :`Mesh` "/Game/Assets/Models/HexTileFlatComplex.HexTileFlatComplex" :`MFiller` "/Game/Assets/Materials/M_HexagonFiller.M_HexagonFiller" :`MBorder` "/Game/Assets/Materials/M_HexagonBorder.M_HexagonBorder")
  (`self.K2_SetActorLocation` (0.0 0.0 0.1)))

(fn `UpdateVisual`
  (params (TileInfo :type "TileInfo Structure") (TileStates :type "Array of ETileState Enum"))
  (bind _tileinfo_pos2d (break `TileInfo` (`local.TileInfo`)))
  (bind _tileinfo_pos2d_2 (break `TileInfo` (`local.TileInfo`)))
  (bind (_tileinfo_pos2d_3 _tileinfo_mappos2d) (break `TileInfo` (`local.TileInfo`)))
  (`/Game/Blueprints/MainMode/GameElements/TileMap/BP_TileMapMeshInst.RemoveInstance` (`self.MeshInst`) _tileinfo_pos2d)
  (`/Game/Blueprints/MainMode/GameElements/TileMap/BP_TileMapMeshInst.AddInstance` (`self.MeshInst`) _tileinfo_pos2d_3 (`KismetMathLibrary.MakeTransform` (`KismetMathLibrary.Conv_Vector2DToVector` _tileinfo_mappos2d)) (`local.TileStates`) (`ActorTileMap.IsTileAccesible` (`self.TileMap`) _tileinfo_pos2d_2)))

(fn `UserConstructionScript`)