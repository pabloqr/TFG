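; Tile map overlay that shows, as floating text, how many turns the player's selected unit needs to reach tiles on its path.
; Binds to BP_TileMap's tile and path events, keeping a position-keyed map of lazily spawned TextRenderActors for accessible tiles.
; Turn counts divide path cost by the unit's current or base movement points, depending on its state.
; TilesInPath tracks labelled tiles for resetting, and ShowTilesInfo toggles the overlay.
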(event `self.ReceiveBeginPlay`
  (bind _returnvalue (`GameplayStatics.GetActorOfClass` "/Game/Blueprints/MainMode/GameElements/TileMap/BP_TileMap.BP_TileMap_C"))
  (bind _output_get (set `self.TileMap` _returnvalue))
  (add `ActorTileMap.OnTileInfoUpdated` _output_get (`|CreateDelegate` :!event `UpdateTextOnTile`))
  (add `ActorTileMap.OnPathCreated` (`self.TileMap`) (`|CreateDelegate` :!event `ResetTilesText`))
  (add `ActorTileMap.OnPathUpdated` (`self.TileMap`) (`|CreateDelegate` :!event `UpdateTextOnTile`)))

(fn `ClearTextActors`
  (bind _values (`BlueprintMapLibrary.Map_Values` (`self.TilesText`)))
  (for _array_element _values
    (`self.K2_DestroyActor` _array_element))
  (`BlueprintMapLibrary.Map_Clear` (`self.TilesText`)))

(fn `DestroyTextActor`
  (params (Pos2D :type "IntPoint Structure"))
  (locals (Actor :type "TextRenderActor Object Reference"))
  (bind _output_get (set `local.Actor` (`BlueprintMapLibrary.Map_Find` (`self.TilesText`) Pos2D)))
  (`/Engine/EditorBlueprintResources/StandardMacros.IsValid` _output_get
    (:`Is Valid`
      (`self.K2_DestroyActor` (`local.Actor`))
      (`BlueprintMapLibrary.Map_Remove` (`self.TilesText`) (`local.Pos2D`)))))

(fn `GetTextActor`
  (params (Pos2D :type "IntPoint Structure"))
  (returns (TextActor :type "TextRenderActor Object Reference"))
  (locals (Actor :type "TextRenderActor Object Reference"))
  (bind _actor (`local.Actor`))
  (bind _textrender (`TextRenderActor.TextRender` (`local.Actor`)))
  (bind _output_get (set `local.Actor` (`BlueprintMapLibrary.Map_Find` (`self.TilesText`) Pos2D)))
  (`/Engine/EditorBlueprintResources/StandardMacros.IsValid` _output_get
    (:`Is Valid`
      (return (`local.Actor`)))
    (:`Is Not Valid`
      ;[0 0 0] Si no se encuentra el actor, se crea y se anade al diccionario de actores
      (bind _returnvalue (`|SpawnActorFromClass` "/Script/Engine.TextRenderActor" (`KismetMathLibrary.MakeTransform` (0.0 0.0 0.0)) "AlwaysSpawn" "OverrideRootScale" null null))
      (bind _output_get_2 (set `local.Actor` _returnvalue))
      (`BlueprintMapLibrary.Map_Add` (`self.TilesText`) (`local.Pos2D`) _output_get_2)
      ;[0 0 0] Se desactiva el metodo tick y las colisiones del actor
      (`self.SetActorTickEnabled` _actor false)
      (`self.SetActorEnableCollision` _actor false)
      ;[0 0 0] Se centra el texto
      (`TextRenderComponent.SetHorizontalAlignment` _textrender "EHTA_Center")
      (`TextRenderComponent.SetVerticalAlignment` _textrender "EVRTA_TextCenter")
      (`TextRenderComponent.SetTextRenderColor` _textrender (make `Color` 0 0 0 1))
      (return (`local.Actor`)))))

(fn `GetTextFromPath`
  (params (Path :type "Array of Movement Structure") (Pos2D :type "IntPoint Structure") (UnitInfo :type "/Game/Blueprints/MainMode/GameElements/Units/UnitInfo Structure"))
  (returns (Text :type String))
  (locals (PathInfo :type "Movement Structure"))
  (bind (_unitinfo_state _unitinfo_movementpoints _unitinfo_basemovementpoints) (break `/Game/Blueprints/MainMode/GameElements/Units/UnitInfo` (`local.UnitInfo`)))
  (bind _returnvalue (`LibraryTileMap.IsTileInPath` Path Pos2D))
  (if (!= _returnvalue -1)
    (bind _output_get (set `local.PathInfo` (`|GetArrayItem` Path _returnvalue)))
    (`BlueprintSetLibrary.Set_Add` (`self.TilesInPath`) (`local.Pos2D`))
    (return (`KismetStringLibrary.Conv_IntToString` (`KismetMathLibrary.FCeil` (/ (`KismetMathLibrary.Conv_IntToDouble` (`.TotalCost` (break `Movement` _output_get))) (`KismetMathLibrary.Conv_IntToDouble` (select `EUnitState` _unitinfo_state :`None` _unitinfo_movementpoints :`WaitingForOrders` _unitinfo_movementpoints :`Sleeping` _unitinfo_movementpoints :`FollowingPath` _unitinfo_movementpoints :`NoMovementPoints` _unitinfo_basemovementpoints :`WaitingForNextTurn` _unitinfo_basemovementpoints))))))
    (else
      (return ""))))

(fn `ResetTilesText`
  (params (Tiles :type "Array of Movement Structure"))
  (bind _tilesinpath (`self.TilesInPath`))
  (if (== (`KismetArrayLibrary.Array_Length` Tiles) 0)
    (bind _result (`BlueprintSetLibrary.Set_ToArray` _tilesinpath))
    (`BlueprintSetLibrary.Set_Clear` _tilesinpath)
    (for _array_element _result
      (`self.UpdateTextOnTile` _array_element))
    (else
      (for _array_element_2 (`local.Tiles`)
        (bind _pos2d (break `Movement` _array_element_2))
        (`BlueprintSetLibrary.Set_Remove` (`self.TilesInPath`) _pos2d)
        (`self.UpdateTextOnTile` _pos2d)))))

(fn `SetShowTilesInfo`
  (params (ShowTilesInfo :type Boolean))
  (bind _output_get (set `self.ShowTilesInfo` ShowTilesInfo))
  (if _output_get
    (bind _keys (`BlueprintMapLibrary.Map_Keys` (`ActorTileMap.TilesInfo` (`self.TileMap`))))
    (for _array_element _keys
      (`self.UpdateTextOnTile` _array_element))
    (else
      (`self.ClearTextActors`))))

(fn `UpdateTextOnTile`
  (params (Pos2D :type "IntPoint Structure"))
  (locals (PlayerController :type "/Game/Blueprints/MainMode/Core/BP_CMain Object Reference") (Actor :type "TextRenderActor Object Reference") (TileInfo :type "TileInfo Structure") (TileText :type String) (PathInfo :type "Movement Structure"))
  (bind _tileinfo (`local.TileInfo`))
  (bind _unit (`CMain.Unit` (`local.PlayerController`)))
  (bind (_value _returnvalue) (`BlueprintMapLibrary.Map_Find` (`ActorTileMap.TilesInfo` (`self.TileMap`)) (`local.Pos2D`)))
  (bind _unitinfo (make `/Game/Blueprints/MainMode/GameElements/Units/UnitInfo` (`ActorUnit.State` _unit) (`ActorUnit.MovementPoints` _unit) (`ActorUnit.BaseMovementPoints` _unit)))
  (if (`self.ShowTilesInfo`)
    (if _returnvalue
      (bind _output_get (set `local.TileInfo` _value))
      (if (`LibraryTileMap.IsTileTypeAccesible` (`.TileType` (break `TileInfo` _output_get)))
        (`|ExecutionSequence`
          (:`then_0`
            (bind _asbp_cmain (cast `/Game/Blueprints/MainMode/Core/BP_CMain` (`GameplayStatics.GetPlayerController` 0)))
            (set `local.PlayerController` _asbp_cmain)
            (`/Engine/EditorBlueprintResources/StandardMacros.IsValid` (`CMain.Unit` (`local.PlayerController`))
              (:`Is Valid`
                (bind _assplayer_main (cast `SPlayerMain` (`Controller.PlayerState` (`local.PlayerController`))))
                (if (`|EnumEquality` (`SPlayerMain.SelectionState` _assplayer_main) "MovingUnit")
                  (bind _text (`self.GetTextFromPath` (`/Game/Blueprints/MainMode/Core/BP_CMain.CurrentPath` (`local.PlayerController`)) (`local.Pos2D`) _unitinfo))
                  (bind _output_get_2 (set `local.TileText` _text))
                  (if (`KismetStringLibrary.IsEmpty` _output_get_2)
                    _)
                  (else
                    (bind _text_2 (`self.GetTextFromPath` (`ActorUnit.Path` (`CMain.Unit` (`local.PlayerController`))) (`local.Pos2D`) _unitinfo))
                    (bind _output_get_3 (set `local.TileText` _text_2))
                    (if (`KismetStringLibrary.IsEmpty` _output_get_3)
                      _))))))
          (:`then_1`
            (bind _textactor (`self.GetTextActor` (`local.Pos2D`)))
            (set `local.Actor` _textactor)
            (`TextRenderComponent.K2_SetText` (`TextRenderActor.TextRender` (`local.Actor`)) (`KismetTextLibrary.Conv_StringToText` (`local.TileText`)))
            (`self.K2_SetActorTransform` (`local.Actor`) (`KismetMathLibrary.MakeTransform` (`KismetMathLibrary.MakeVector` (+ (`KismetMathLibrary.BreakVector2D` (`.MapPos2D` (break `TileInfo` _tileinfo))) 0.0) (`.Y` (`KismetMathLibrary.BreakVector2D` (`.MapPos2D` (break `TileInfo` _tileinfo)))) 15.0) (struct :`Pitch` 90.0 :`Yaw` 90.0) (2.0 2.0 2.0)) false false)))
        (else
          (`self.DestroyTextActor` (`local.Pos2D`) :!label _label)))
      (else
        (goto _label)))))

(fn `UserConstructionScript`)