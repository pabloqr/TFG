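; BP_CMainAI is the main mode's AI class that hands play to the next turn once its own turn can finish.
; When OnTurnFinished fires, a short looping timer polls CanFinishTurn and prints the result to screen for debugging.
; Once the check passes, it clears the timer and calls NextTurn on the BP_MMain game mode.
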(event `self.ReceiveBeginPlay`
  (add `self.OnTurnFinished` (delegate `EventOnTurnFinished`)))

(event `EventOnTurnFinished`
  (bind _returnvalue (`KismetSystemLibrary.K2_SetTimerDelegate` (delegate `EventCheckForTurnFinish`) 0.3 true)))

(event `EventCheckForTurnFinish`
  (bind _returnvalue (`self.CanFinishTurn`))
  (`KismetSystemLibrary.PrintString` (`KismetStringLibrary.Conv_BoolToString` _returnvalue))
  (if _returnvalue
    (`KismetSystemLibrary.K2_ClearAndInvalidateTimerHandle` (stale `EventOnTurnFinished` _returnvalue))
    (bind _asbp_mmain (cast `/Game/Blueprints/MainMode/Core/BP_MMain` (`GameplayStatics.GetGameMode`)))
    (`MMain.NextTurn` _asbp_mmain)))

(fn `UserConstructionScript`)