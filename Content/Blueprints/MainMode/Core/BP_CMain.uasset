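; Main-mode player controller that handles mouse input for selecting, spawning and moving units on the BP_TileMap found at BeginPlay.
; Left click selects the unit on the tile under the cursor, or spawns a BP_MilitaryUnit on a valid, accessible empty tile and registers it with the player's BP_PFaction pawn.
; Right click gets a tile map path to the cursor tile and hands it to the selected unit to follow.
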(event `self.ReceiveBeginPlay`
  (set `self.bShowMouseCursor` true)
  (`self.EnableInput` self)
  (bind _returnvalue (`GameplayStatics.GetActorOfClass` "/Game/Blueprints/MainMode/GameElements/BP_TileMap.BP_TileMap_C"))
  (set `self.TileMap` _returnvalue))

(event `self.ReceiveTick`
  (params (DeltaSeconds :type "Float (single-precision)")))

(event `Key|LeftMouseButton`
  (params (Key :type "Key Structure"))
  (:`Pressed`
    (`KismetSystemLibrary.PrintString` "Left" false)
    (`self.GetUnitUnderCursor`)))

(event `Key|RightMouseButton`
  (params (Key :type "Key Structure"))
  (:`Pressed`
    (`KismetSystemLibrary.PrintString` "Right" false)
    (`self.MoveSelectedUnit`)))

(fn `AssignPathToUnit`
  (params (Path :type "Array of Movement Structure"))
  (bind _unit (`self.Unit`))
  (bind _output_get (set `ActorUnit.Path` Path _unit))
  (set `ActorUnit.State` "FollowingPath" _unit)
  (for _array_element _output_get
    (`KismetSystemLibrary.PrintString` (`KismetStringLibrary.Conv_IntPointToString` (break `Movement` _array_element)) false)))

(fn `GetUnitUnderCursor`
  (locals (CurrPos2D :type "IntPoint Structure") (CurrMapPos2D :type "Vector2D Structure"))
  (bind (_currmappos2d_x _currmappos2d_y) (`KismetMathLibrary.BreakVector2D` (`local.CurrMapPos2D`)))
  (bind _tilemap (`self.TileMap`))
  (bind _selectedtile (`/Game/Blueprints/MainMode/GameElements/BP_TileMap.GetTileUnderCursor` (`self.TileMap`)))
  (bind _output_get (set `self.Tile` _selectedtile))
  (set `local.CurrPos2D` (`ActorPlaceableElement.Pos2D` _output_get))
  (set `local.CurrMapPos2D` (`ActorPlaceableElement.MapPos2D` _output_get))
  (if (`ActorTile.HasUnit` (`self.Tile`))
    (set `self.Unit` (`ActorTile.Unit` (`self.Tile`)))
    (else
      (bind _returnvalue (`ActorTileMap.CheckValidPosition` (`self.TileMap`) (`local.CurrPos2D`) (make `IntPoint` (`ActorTileMap.Rows` _tilemap) (`ActorTileMap.Cols` _tilemap))))
      (if (and _returnvalue (`ActorTile.IsAccesible` (`self.Tile`)))
        (bind _returnvalue_2 (`|SpawnActorFromClass` "/Game/Blueprints/MainMode/GameElements/Units/BP_MilitaryUnit.BP_MilitaryUnit_C" (`KismetMathLibrary.MakeTransform` (`KismetMathLibrary.MakeVector` _currmappos2d_x _currmappos2d_y)) "Undefined" "OverrideRootScale" null null))
        (bind _output_get_2 (set `self.Unit` _returnvalue_2))
        (set `ActorTile.Unit` _output_get_2 (`self.Tile`))
        (set `ActorPlaceableElement.Pos2D` (`ActorPlaceableElement.Pos2D` (`self.Tile`)) (`self.Unit`))
        (bind _asbp_pfaction (cast `/Game/Blueprints/MainMode/Core/BP_PFaction` (`GameplayStatics.GetPlayerPawn` 0)))
        (`KismetArrayLibrary.Array_AddUnique` (`PawnFaction.Units` _asbp_pfaction) (`self.Unit`))))))

(fn `MoveSelectedUnit`
  (`/Engine/EditorBlueprintResources/StandardMacros.IsValid` (`self.Unit`)
    (:`Is Valid`
      (bind _selectedtile (`/Game/Blueprints/MainMode/GameElements/BP_TileMap.GetTileUnderCursor` (`self.TileMap`)))
      (bind _returnvalue (`ActorTileMap.FindPath` (`self.TileMap`) (`ActorPlaceableElement.Pos2D` (`self.Unit`)) (`ActorPlaceableElement.Pos2D` _selectedtile)))
      (for _array_element _returnvalue
        (`KismetSystemLibrary.PrintString` (`KismetStringLibrary.Conv_IntPointToString` (break `Movement` _array_element)) false)
        (`ActorUnit.AssignPath` (`self.Unit`) _returnvalue)
        (`ActorUnit.ContinuePath` (`self.Unit`))))))

(fn `UserConstructionScript`)