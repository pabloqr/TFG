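; Main game mode that sets up a turn-based match on a tile map with one player faction and AI factions.
; BeginPlay spawns the tile map and caches the game state, binding an event to an init-finished delegate.
; Once parameters initialize, it registers the player pawn's faction, spawns the AI factions, then starts the next turn.
; Each faction receives a civil unit and infantry on generated starting tiles keyed by faction index.
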(event `self.ReceiveBeginPlay`
  (add `self.OnInitFinished` (`|CreateDelegate` :!event `OnParamsInitFinished`))
  (bind _returnvalue (`|SpawnActorFromClass` "/Game/Blueprints/Core/GameElements/TileMap/BP_TileMap.BP_TileMap_C" (`KismetMathLibrary.MakeTransform` (0.0 0.0 0.0)) "AlwaysSpawn" "OverrideRootScale" null null))
  (set `self.TileMap` _returnvalue)
  (bind _asbp_smain (cast `/Game/Blueprints/MainMode/Core/BP_SMain` (`GameplayStatics.GetGameState`)))
  (set `self.StateMain` _asbp_smain))

(event `OnParamsInitFinished`
  (bind _returnvalue (`ActorTileMap.GenerateStartingPositions` (`self.TileMap`) (`SMain.NumFactions` (`self.StateMain`))))
  (set `self.Positions` _returnvalue)
  (bind _asbp_pfaction (cast `/Game/Blueprints/MainMode/Core/BP_PFaction` (`GameplayStatics.GetPlayerPawn` 0)))
  (`self.InitFaction` _asbp_pfaction _returnvalue)
  (`self.CreateAIFactions` _returnvalue)
  (`self.NextTurn`))

(fn `CreateAIFactions`
  (params (InitialPositions :type "Map of Integer to TilesArray Structure"))
  (locals (FactionIndex :type Integer))
  (for _index (range 1 (`SMain.NumFactions` (`self.StateMain`)))
    (set `local.FactionIndex` _index)
    (bind _returnvalue (`AIBlueprintHelperLibrary.SpawnAIFromClass` "/Game/Blueprints/MainMode/Core/BP_PFaction.BP_PFaction_C" null (0.0 0.0 0.0) (struct) false null))
    (bind _asbp_pfaction (cast `/Game/Blueprints/MainMode/Core/BP_PFaction` _returnvalue))
    (set `PawnFaction.Index` (`local.FactionIndex`) _asbp_pfaction)
    (`self.InitFaction` _asbp_pfaction (`local.InitialPositions`))))

(fn `InitFaction`
  (params (Faction :type "PawnFaction Object Reference") (InitialPositions :type "Map of Integer to TilesArray Structure"))
  (locals (Pos :type "IntPoint Structure"))
  (bind _index (`PawnFaction.Index` (`local.Faction`)))
  (bind (_value _returnvalue) (`BlueprintMapLibrary.Map_Find` (`local.InitialPositions`) _index))
  (`SMain.AddFaction` (`self.StateMain`) Faction)
  (if (> (`BlueprintMapLibrary.Map_Length` InitialPositions) 0)
    ;[0 0 0] Se generan las unidades iniciales de la faccion
    (`KismetSystemLibrary.PrintString` (`KismetStringLibrary.Conv_IntToString` _index))
    (if _returnvalue
      (for (_array_element _array_index) (`.TilesArray` (break `TilesArray` _value))
        (bind _output_get (set `local.Pos` _array_element))
        (`KismetSystemLibrary.PrintString` (`KismetStringLibrary.Conv_IntPointToString` _output_get))
        (`/Game/Blueprints/Core/GameElements/TileMap/BP_TileMap.InitUnit` (`self.TileMap`) (`local.Faction`) (`local.Pos`) (`|GetArrayItem` (`|MakeArray` (make `ProductionElement` :`Unit` "/Game/Blueprints/MainMode/GameElements/Units/BP_CivilUnit.BP_CivilUnit_C" :`UnitType` "Civil") (make `ProductionElement` :`Unit` "/Game/Blueprints/MainMode/GameElements/Units/BP_MilitaryUnit.BP_MilitaryUnit_C" :`UnitType` "Infantry")) _array_index))))))

(fn `UserConstructionScript`)