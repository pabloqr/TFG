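; BP_MilitaryUnit is a military unit actor that moves between tiles on the map.
; On BeginPlay it caches the BP_TileMap and binds to the OnUnitMoved event.
; A move plays the UnitMovement timeline, lerping from the actor's current location, re-read each update, toward the destination tile's 2D map position.
; The same event also clears the previous tile's Unit reference and assigns it to the new tile.
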(event `self.ReceiveBeginPlay`
  (bind _returnvalue (`GameplayStatics.GetActorOfClass` "/Game/Blueprints/MainMode/BP_TileMap.BP_TileMap_C"))
  (set `self.TileMap` _returnvalue)
  (add `ActorUnit.OnUnitMoved` (`|CreateDelegate` :!event `EventOnUnitMoved`)))

(event `EventOnUnitMoved`
  (params (PrevPos :type "IntPoint Structure") (CurrPos :type "IntPoint Structure") (Unit :type "ActorUnit Object Reference"))
  (bind _tilemap (`self.TileMap`))
  (bind _output (`|GetArrayItem` (`ActorTileMap.TilesInfo` (`self.TileMap`)) (`self.CurrentTileIndex`)))
  (`|ExecutionSequence`
    (:`then_0`
      (set `self.CurrentTileIndex` (`ActorTileMap.GetPositionInArray` (`self.TileMap`) CurrPos))
      (bind (_direction _locationalpha) (`Timeline|UnitMovement`)
        (:`Update`
          (`self.K2_SetActorLocationAndRotation` (`KismetMathLibrary.VLerp` (`self.K2_GetActorLocation`) (`KismetMathLibrary.MakeVector` (`KismetMathLibrary.BreakVector2D` (`.MapPos2D` (break `TileInfo` _output))) (`.Y` (`KismetMathLibrary.BreakVector2D` (`.MapPos2D` (break `TileInfo` _output))))) _locationalpha)))))
    (:`then_1`
      (set `ActorTile.Unit` null (`|GetArrayItem` (`ActorTileMap.Tiles` _tilemap) (`ActorTileMap.GetPositionInArray` _tilemap PrevPos)))
      (set `ActorTile.Unit` Unit (`|GetArrayItem` (`ActorTileMap.Tiles` (`self.TileMap`)) (`self.CurrentTileIndex`))))))

(fn `UserConstructionScript`)