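; Mountain hex tile Blueprint that randomizes its appearance at BeginPlay before calling the parent's logic.
; SelectMesh picks one of two mountain meshes with its matching material.
; DisplayForest scatters a random number of small, randomly rotated and scaled tree instances through the Trees component.
; Placement uses polar coordinates with a square-root radius, confining trees to a partial ring around the tile's origin rather than the whole tile.
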(event `self.ReceiveBeginPlay`
  (`self.SelectMesh`)
  (`self.DisplayForest`)
  (`parent.ReceiveBeginPlay`))

(fn `DisplayForest`
  (locals (Radius :type "Float (double-precision)") (Alpha :type "Float (double-precision)"))
  (bind _returnvalue (`KismetMathLibrary.RandomFloatInRange` 0.5 0.9))
  (for _ (range (+ (`KismetMathLibrary.RandomIntegerInRange` 70 150) 1))
    (bind _output_get (set `local.Radius` (* (`KismetMathLibrary.Sqrt` _returnvalue) 80.0)))
    (bind _output_get_2 (set `local.Alpha` (* _returnvalue 2.0 (`KismetMathLibrary.GetPI`))))
    (`InstancedStaticMeshComponent.AddInstance` (`self.Trees`) (`KismetMathLibrary.MakeTransform` (`KismetMathLibrary.MakeVector` (* (`KismetMathLibrary.Cos` _output_get_2) _output_get) (* (`KismetMathLibrary.Sin` _output_get_2) _output_get)) (`KismetMathLibrary.MakeRotator` 0.0 0.0 (`KismetMathLibrary.RandomFloatInRange` 0.0 360.0)) (`KismetMathLibrary.Conv_DoubleToVector` (`KismetMathLibrary.RandomFloatInRange` 0.01 0.02))))))

(fn `SelectMesh`
  (bind _tilemesh (`self.TileMesh`))
  (switch `int` (`KismetMathLibrary.RandomIntegerInRange` 0 1)
    (:`0`
      (`StaticMeshComponent.SetStaticMesh` _tilemesh "/Game/Assets/Models/HexMountainTile_0.HexMountainTile_0")
      (`PrimitiveComponent.SetMaterial` _tilemesh 0 "/Game/Assets/Materials/M_Mountain_0.M_Mountain_0"))
    (:`1`
      (`StaticMeshComponent.SetStaticMesh` _tilemesh "/Game/Assets/Models/HexMountainTile_1.HexMountainTile_1")
      (`PrimitiveComponent.SetMaterial` _tilemesh 0 "/Game/Assets/Materials/M_Mountain_1.M_Mountain_1"))))

(fn `UserConstructionScript`
  (`parent.UserConstructionScript`))