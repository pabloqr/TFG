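; BP_Tile_Mountains is a mountain hex tile that randomizes its appearance when play begins.
; On BeginPlay, SelectMesh randomly picks one of two mountain meshes and sets its matching material on TileMesh, then the parent's BeginPlay runs.
; The construction script only calls the parent, and the click handler on TileMesh is empty.
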(event `self.ReceiveBeginPlay`
  (`self.SelectMesh`)
  (`parent.ReceiveBeginPlay`))

(event `self.TileMesh.OnClicked`
  (params (TouchedComponent :type "PrimitiveComponent Object Reference") (ButtonPressed :type "Key Structure")))

(fn `SelectMesh`
  (bind _tilemesh (`self.TileMesh`))
  (switch `int` (`KismetMathLibrary.RandomIntegerInRange` 0 1)
    (:`0`
      (`StaticMeshComponent.SetStaticMesh` _tilemesh "/Game/Assets/Models/HexMountainTile_0.HexMountainTile_0")
      (`PrimitiveComponent.SetMaterial` _tilemesh 0 "/Game/Assets/Materials/M_Mountain_0.M_Mountain_0"))
    (:`1`
      (`StaticMeshComponent.SetStaticMesh` _tilemesh "/Game/Assets/Models/HexMountainTile_1.HexMountainTile_1")
      (`PrimitiveComponent.SetMaterial` _tilemesh 0 "/Game/Assets/Materials/M_Mountain_1.M_Mountain_1"))))

(fn `UserConstructionScript`
  (`parent.UserConstructionScript`))