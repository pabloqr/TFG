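; Editor-mode controller that handles mouse hover and selection of tiles on the level's BP_TileMap.
; Each tick it queries the tile under the cursor and moves the Hovered state between tiles.
; Left click clears the previous selection and path, neighbor and reachable highlights, marks the hovered tile Selected and broadcasts its type.
; Helpers select by position and draw CurrentPath; right click only prints debug text.
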(event `self.ReceiveBeginPlay`
  (set `self.bShowMouseCursor` true)
  (`self.EnableInput` self)
  (bind _returnvalue (`GameplayStatics.GetActorOfClass` "/Game/Blueprints/Core/GameElements/TileMap/BP_TileMap.BP_TileMap_C"))
  (set `self.TileMap` _returnvalue))

(event `self.ReceiveTick`
  (params (DeltaSeconds :type "Float (single-precision)"))
  (`self.UpdateTileUnderCursor`))

(event `Key|LeftMouseButton`
  (params (Key :type "Key Structure"))
  (:`Pressed`
    (`KismetSystemLibrary.PrintString` "Left" false)
    (`self.SelectTile`)))

(event `Key|RightMouseButton`
  (params (Key :type "Key Structure"))
  (:`Pressed`
    (`KismetSystemLibrary.PrintString` "Right pressed" false))
  (:`Released`
    (`KismetSystemLibrary.PrintString` "Right released" false)))

(fn `DrawPath`
  (for _array_element (`self.CurrentPath`)
    (bind _returnvalue (`ActorTileMap.GetTileAtPos` (`self.TileMap`) (break `Movement` _array_element)))
    (`/Game/Blueprints/Core/GameElements/TileMap/BP_TileMap.AddStateToTile` (`self.TileMap`) _returnvalue (`|MakeArray` "InPath" :!type "ETileState Enum"))))

(fn `SelectTile`
  (bind (_info_pos2d _info_mappos2d _info_type) (break `TileInfo` (`ActorTile.Info` (`self.SelectedTile`))))
  (`self.UnselectTile`)
  (`self.UpdateTileUnderCursor`)
  (`/Engine/EditorBlueprintResources/StandardMacros.IsValid` (`self.HoveredTile`)
    (:`Is Valid`
      (bind _output_get (set `self.SelectedTile` (`self.HoveredTile`)))
      (`/Game/Blueprints/Core/GameElements/TileMap/BP_TileMap.AddStateToTile` (`self.TileMap`) _output_get (`|MakeArray` "Selected" :!type "ETileState Enum"))
      (`self.OnSelectedTileUpdated` _info_type))))

(fn `UnselectTile`
  (bind _tilemap (`self.TileMap`))
  (`/Engine/EditorBlueprintResources/StandardMacros.IsValid` (`self.SelectedTile`)
    (:`Is Valid`
      (`/Game/Blueprints/Core/GameElements/TileMap/BP_TileMap.RemoveStateFromTile` (`self.TileMap`) (`self.SelectedTile`) (`|MakeArray` "Selected" :!type "ETileState Enum")))
    (:`Is Not Valid`
      _))
  ;[0 0 0] Se limpian los estados de las casillas
  (`/Game/Blueprints/Core/GameElements/TileMap/BP_TileMap.ClearStateFromTiles` _tilemap "InPath")
  (`/Game/Blueprints/Core/GameElements/TileMap/BP_TileMap.ClearStateFromTiles` _tilemap "Neighbor")
  (`/Game/Blueprints/Core/GameElements/TileMap/BP_TileMap.ClearStateFromTiles` _tilemap "Reachable")
  (set `self.SelectedTile` null)
  ;[0 0 0] Se actualiza el color de la casilla
  (`/Game/Blueprints/Core/GameElements/TileMap/BP_TileMap.UpdateTileVisual` (`self.TileMap`) (`self.HoveredTile`))
  (`self.OnSelectedTileUpdated` "None"))

(fn `UpdateSelectedTile`
  (params (Pos :type "IntPoint Structure"))
  (bind _tilemap (`self.TileMap`))
  (bind _returnvalue (`ActorTileMap.GetPositionInArray` _tilemap Pos))
  (if (!= _returnvalue -1)
    (bind _output_get (set `self.SelectedTile` (`|GetArrayItem` (`ActorTileMap.Tiles` _tilemap) _returnvalue)))
    (`/Game/Blueprints/Core/GameElements/TileMap/BP_TileMap.AddStateToTile` (`self.TileMap`) _output_get (`|MakeArray` "Selected" :!type "ETileState Enum"))))

(fn `UpdateTileUnderCursor`
  (locals (CurrTile :type "/Game/Blueprints/Core/GameElements/Tiles/BP_Tile Object Reference") (CurrElement :type "ActorDamageableElement Object Reference"))
  (bind _array (`|MakeArray` "Hovered" :!type "ETileState Enum"))
  (bind _hoveredtile (`self.HoveredTile`))
  (bind _hoveredtile_2 (`self.HoveredTile`))
  (bind _tile (`/Game/Blueprints/Core/GameElements/TileMap/BP_TileMap.GetTileUnderCursor` (`self.TileMap`)))
  (`/Engine/EditorBlueprintResources/StandardMacros.IsValid` _tile
    (:`Is Valid`
      ;[0 0 0] Si hay una casilla bajo el cursor, se verifica que sea diferente a la anterior y se actualiza el estado de la actual y la anterior. Se comprueba si hay una unidad debajo y si es amiga o enemiga
      (bind _output_get (set `local.CurrTile` _tile))
      (if (!= _output_get (`self.HoveredTile`))
        (`/Engine/EditorBlueprintResources/StandardMacros.IsValid` _hoveredtile
          (:`Is Valid`
            (`/Game/Blueprints/Core/GameElements/TileMap/BP_TileMap.RemoveStateFromTile` (`self.TileMap`) _hoveredtile _array))
          (:`Is Not Valid`
            _))
        (`/Game/Blueprints/Core/GameElements/TileMap/BP_TileMap.AddStateToTile` (`self.TileMap`) (`local.CurrTile`) _array)
        (set `self.HoveredTile` (`local.CurrTile`))))
    (:`Is Not Valid`
      ;[0 0 0] Si no hay ninguna casilla bajo el cursor, se elimina el estado de la casilla anterior y se establece a null
      (`/Engine/EditorBlueprintResources/StandardMacros.IsValid` _hoveredtile_2
        (:`Is Valid`
          (`/Game/Blueprints/Core/GameElements/TileMap/BP_TileMap.RemoveStateFromTile` (`self.TileMap`) _hoveredtile_2 (`|MakeArray` "Hovered" :!type "ETileState Enum"))
          (set `self.HoveredTile` null))))))

(fn `UserConstructionScript`)